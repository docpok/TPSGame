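; BP_Loot is a world pickup for an inventory item and amount, defined by a DT_Item row.
; On authority, its construction script validates the item and amount, then applies the pickup mesh and transform corrections.
; Interaction messages toggle a key prompt widget, update the remaining amount, or ask the interacting actor to destroy empty loot.
; DoSaveLoot writes its state to the save object by display name, unless IgnoreSaving is set.
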(event Custom|RefreshInteract
  (params (Key :type Text) (Amount :type Integer))
  ;[1 1 1] Refresh interact text
  (bind _asw_interact (Utilities|Casting|CastToW_Interact (UserInterface|GetUserWidgetObject (Variables|Default|GetWidget))))
  (Default|UpdateKey _asw_interact Key (Utilities|Text|FormatText "to pick-up ({Amount} {Name})" Amount (Variables|Spawn|GetItemName))))

(event EventBeginPlay
  ;[1 1 1] Hide debug text
  (Rendering|SetVisibility (Variables|Default|GetTextRender) false false)
  (bind _returnvalue (Utilities|GetDataTableRow "/Game/AntizeInventory/Logics/Datatable/DT_Item.DT_Item" (.RowName (Utilities|Struct|BreakDataTableRowHandle (Utilities|Struct|BreakS_InventorySlot (Variables|Setting|GetItemOnLoot)))))
    (:then
      (Variables|Spawn|SetItemName (Utilities|Struct|BreakS_Item _returnvalue)))))

(event EventMSGInteraction
  (params (Interaction :type E_Interaction%20Enum :default "NewEnumerator0") (Amount :type Integer) (FromActor :type Actor%20Object%20Reference) (Key :type Text))
  (bind _widget (Variables|Default|GetWidget))
  ;[1 1 1] Show/Hide Interact text
  (switch Utilities|FlowControl|Switch|SwitchonE_Interaction Interaction
    (:NewEnumerator0
      (Rendering|SetVisibility _widget true false)
      (CallFunction|RefreshInteract Key (Utilities|Struct|BreakS_InventorySlot (Variables|Setting|GetItemOnLoot))))
    (:NewEnumerator1
      (Rendering|SetVisibility _widget false false))
    (:NewEnumerator2
      ;;[1 1 1] If Loot is empty call destroy in ActorRef
      (if (> Amount 0)
        (Utilities|Struct|SetmembersinS_InventorySlot (Variables|Setting|GetItemOnLoot) Amount)
        (else
          (Class|BPInventoryInterface|MSGDestroyActor(Message) FromActor self))))))

(fn ConstructionScript
  (bind _itemonloot (Variables|Setting|GetItemOnLoot))
  (bind _interactcorrection (Variables|Setting|GetInteractCorrection))
  (bind (_location _rotation _scale) (Utilities|Struct|BreakS_Correction _interactcorrection))
  (Networking|SwitchHasAuthority
    (:Authority
      ;[1 1 1] If item not found, get the first item
      (bind _returnvalue (Utilities|GetDataTableRow "/Game/AntizeInventory/Logics/Datatable/DT_Item.DT_Item" (.RowName (Utilities|Struct|BreakDataTableRowHandle (Utilities|Struct|BreakS_InventorySlot (Variables|Setting|GetItemOnLoot)))))
        (:then
          _)
        (:RowNotFound
          (bind _outrownames (DataTable|GetDataTableRowNames "/Game/AntizeInventory/Logics/Datatable/DT_Item.DT_Item"))
          (Utilities|Struct|SetmembersinS_InventorySlot _itemonloot (Utilities|Struct|MakeDataTableRowHandle "/Game/AntizeInventory/Logics/Datatable/DT_Item.DT_Item" (Utilities|Array|Get(acopy) _outrownames)))))
      ;[1 1 1] Set minimum of amount to 1
      (if (> (Utilities|Struct|BreakS_InventorySlot _itemonloot) 0)
        _
        (else
          (Utilities|Struct|SetmembersinS_InventorySlot (Variables|Setting|GetItemOnLoot) 1)))
      (Components|StaticMesh|SetStaticMesh (Variables|Default|GetLoot_Mesh) (.PickupMesh (Utilities|Struct|BreakS_Item _returnvalue)))
      (Transformation|SetRelativeTransform (Variables|Default|GetLoot_Mesh) (Math|Transform|MakeTransform (.Location (Utilities|Struct|BreakS_Correction (.MeshCorrection (Utilities|Struct|BreakS_Item _returnvalue)))) (.Rotation (Utilities|Struct|BreakS_Correction (.MeshCorrection (Utilities|Struct|BreakS_Item _returnvalue)))) (.Scale (Utilities|Struct|BreakS_Correction (.MeshCorrection (Utilities|Struct|BreakS_Item _returnvalue))))) false false)
      (Transformation|AddRelativeRotation (Variables|Default|GetArrow) (Variables|Setting|GetMeshRotCorrection) false false)
      (Transformation|SetRelativeTransform (Variables|Default|GetInteract) (Math|Transform|MakeTransform _location _rotation _scale) false false)
      (Transformation|SetRelativeLocation (Variables|Default|GetWidget) (Variables|Setting|GetPickUpTextLocCorrection) false false))))

(fn DoSaveLoot
  (params (SaveRef :type BP%20Save%20Inventory%20Object%20Reference) (LootName :type Array%20of%20Strings))
  (LocalVariables|SetLocal_Save SaveRef)
  (if (not (Variables|Setting|GetIgnoreSaving?))
    (LocalVariables|SetLocal_SaveLoot (Utilities|Struct|MakeS_SaveLoot (Utilities|GetDisplayName self) (Variables|Setting|GetItemOnLoot)))
    (bind _output_get (LocalVariables|SetLocal_FindIndex (Utilities|Array|FindItem LootName (Utilities|GetDisplayName self))))
    (if (>= _output_get 0)
      (Utilities|Array|SetArrayElem (Variables|/Game/AntizeInventory/Blueprints/SaveGame/BP_SaveInventory.BP_SaveInventory_C|GetSave_Loot (LocalVariables|GetLocal_Save)) (LocalVariables|GetLocal_FindIndex) (LocalVariables|GetLocal_SaveLoot) true)
      (else
        (Utilities|Array|Add (Variables|/Game/AntizeInventory/Blueprints/SaveGame/BP_SaveInventory.BP_SaveInventory_C|GetSave_Loot (LocalVariables|GetLocal_Save)) (LocalVariables|GetLocal_SaveLoot))))
    (return)
    (else
      (return))))

(fn MSGGetDestroyedLoot
  (return 0))

(fn MSGGetEquippedWeapon
  (return ""))

(fn MSGGetInventory
  (return 0))

(fn MSGGetStats
  (return 0.0 0.0 0.0))