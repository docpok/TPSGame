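; BP_Cible is a shooting target that takes BP_Projectile hits, falls when its life runs out and stands back up.
; Head and Body hits feed a server-authority TakeDamage, which adds random variance, weights headshots higher and has the shooting character show the damage.
; At zero life, a DoOnce gate disables collision, tips the Porteur component over via a timeline, then restores life, pose and collision after a delay.
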(event OnComponentHit(Head)
  (params (HitComponent :type Primitive%20Component%20Object%20Reference) (OtherActor :type Actor%20Object%20Reference) (OtherComp :type Primitive%20Component%20Object%20Reference) (NormalImpulse :type Vector :default "0, 0, 0") (Hit :type Hit%20Result%20Structure%20%28by%20ref%29))
  ;[1 1 1] On Hit with Projectile
  (bind _asbp_projectile (Utilities|Casting|CastToBP_Projectile OtherActor))
  (CallFunction|TakeDamage (Variables|/Game/AntizeInventory/Blueprints/Other/BP_Projectile.BP_Projectile_C|GetDamage _asbp_projectile) true (Variables|/Game/AntizeInventory/Blueprints/Other/BP_Projectile.BP_Projectile_C|GetOwnerRef _asbp_projectile)))

(event OnComponentHit(Body)
  (params (HitComponent :type Primitive%20Component%20Object%20Reference) (OtherActor :type Actor%20Object%20Reference) (OtherComp :type Primitive%20Component%20Object%20Reference) (NormalImpulse :type Vector :default "0, 0, 0") (Hit :type Hit%20Result%20Structure%20%28by%20ref%29))
  ;[1 1 1] On Hit with Projectile
  (bind _asbp_projectile (Utilities|Casting|CastToBP_Projectile OtherActor))
  (CallFunction|TakeDamage (Variables|/Game/AntizeInventory/Blueprints/Other/BP_Projectile.BP_Projectile_C|GetDamage _asbp_projectile) false (Variables|/Game/AntizeInventory/Blueprints/Other/BP_Projectile.BP_Projectile_C|GetOwnerRef _asbp_projectile)))

(event Custom|Anim
  ;[1 1 1] Anim if life is down of 0 and reset after a moment
  (bind _alpha (Timeline|Timeline_0 PlayFromStart)
    (:Update
      (Transformation|SetRelativeRotation (Variables|Default|GetPorteur) (select (<= (Variables|Traitement|GetLife) 0.0) (Math|Rotator|Lerp(Rotator) "0, 0, 0" "0, 0,90.000000" _alpha) (Math|Rotator|Lerp(Rotator) "0, 0,90.000000" "0, 0, 0" _alpha)) false false))))

(event Custom|TakeDamage
  (params (DamageBrut :type Float%20%28single-precision%29) (Head? :type Boolean) (OwnerRef :type Actor%20Object%20Reference))
  ;[1 1 1] On Hit with Projectile
  (Networking|SwitchHasAuthority
    (:Authority
      (Variables|Traitement|SetDamage (* (+ DamageBrut (Math|Random|RandomFloatinRange (* DamageBrut 0.01) (* DamageBrut 0.05))) (select Head? 1.5e+02 1e+02)))
      (Variables|Traitement|SetLife (- (Variables|Traitement|GetLife) (Variables|Traitement|GetDamage)))
      (bind _asbp_my_character (Utilities|Casting|CastToBP_MyCharacter OwnerRef)
        (:then
          (Default|ShowDamage _asbp_my_character (Transformation|GetWorldTransform (Variables|Default|GetWidget)) (Variables|Traitement|GetDamage)))
        (:CastFailed
          _))
      ;[1 1 1] Anim if life is down of 0 and reset after a moment
      (if (<= (Variables|Traitement|GetLife) 0.0)
        (Utilities|FlowControl|DoOnce false :!label _label
          (:Completed
            (Collision|SetCollisionEnabled (Variables|Default|GetBody) "NoCollision")
            (CallFunction|Anim)
            (Utilities|FlowControl|Delay 5.0)
            (Variables|Traitement|SetLife (Variables|Setting|GetMaxLife))
            (CallFunction|Anim)
            (Collision|SetCollisionEnabled (Variables|Default|GetBody) "QueryAndPhysics")
            (goto _label Reset)))))))

(fn ConstructionScript
  (Variables|Traitement|SetLife (Variables|Setting|GetMaxLife)))