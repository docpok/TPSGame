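; Player controller for the inventory system that owns the player HUD and relays interface messages.
; On BeginPlay, the local controller creates the HUD widget and adds it to the viewport, and incoming show-message calls feed it interaction results.
; Inventory and equipped-weapon queries pass through to the controlled pawn when it is valid.
; The destroyed-loot and stats getters are stubs returning empty or zero values.
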(event EventBeginPlay
  ;[1 1 1] Constructeur
  (if (Pawn|IsLocalPlayerController)
    ;;[1 1 1] Create player HUD
    (bind _returnvalue (UserInterface|CreateWidget "/Game/AntizeInventory/Widgets/W_PlayerHUD.W_PlayerHUD_C"))
    (bind _output_get (Variables|Spawn|SetPlayerHUDRef _returnvalue))
    (UserInterface|Viewport|AddtoViewport _output_get 2)))

(event EventMSGShowMessage
  (params (Messages :type Text))
  ;[1 1 1] Show Message
  (Default|AddInteractResult (Variables|Spawn|GetPlayerHUDRef) Messages))

(fn ConstructionScript)

(fn MSGGetDestroyedLoot
  (return 0))

(fn MSGGetEquippedWeapon
  (bind _returnvalue (Pawn|GetControlledPawn))
  (Utilities|IsValid _returnvalue
    (:Is%20Valid
      (bind _equippedweapon (Class|BPInventoryInterface|MSGGetEquippedWeapon(Message) _returnvalue))
      (return _equippedweapon))
    (:Is%20Not%20Valid
      (return ""))))

(fn MSGGetInventory
  (bind _returnvalue (Pawn|GetControlledPawn))
  (Utilities|IsValid _returnvalue
    (:Is%20Valid
      (bind _inventoryref (Class|BPInventoryInterface|MSGGetInventory(Message) _returnvalue))
      (return _inventoryref))
    (:Is%20Not%20Valid
      (return 0))))

(fn MSGGetStats
  (return 0.0 0.0 0.0))