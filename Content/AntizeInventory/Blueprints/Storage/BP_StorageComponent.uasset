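; Storage container component that holds a fixed-size array of item slots exchanged with the inventory.
; Deposits and in-storage moves resolve items through DT_Item, then merge stacks, swap or move slots and refresh the affected widgets.
; Depositing the equipped weapon's slot also unequips it through a character message.
; Contents save and load as one entry in the save object's storage array, indexed by StorageName converted to an integer.
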(event EventBeginPlay
  (Utilities|Array|Resize (Variables|Traitement|GetStorageSlots) (Variables|Spawn|GetStorageSize)))

(fn GetItematIndex
  (params (Index :type Integer))
  (bind _storageslots (Variables|Traitement|GetStorageSlots))
  (bind _output (Utilities|Array|Get(acopy) _storageslots Index))
  (bind (_item _amount _ammo) (Utilities|Struct|BreakS_InventorySlot _output))
  (bind _returnvalue (Utilities|GetDataTableRow "/Game/AntizeInventory/Logics/Datatable/DT_Item.DT_Item" (.rowname _item))
    (:then
      (return (<= _amount 0) _returnvalue _amount _ammo (Utilities|Struct|BreakS_WeaponCharacteristics (Utilities|Struct|BreakS_Item _returnvalue))))
    (:RowNotFound
      (return true "" 0 0 0))))

(fn AddItemtoStorage
  (params (StorageIndex :type Integer) (InventoryIndex :type Integer))
  (bind _inventoryref (Variables|Spawn|GetInventoryRef))
  (bind _inventoryslots (Variables|/Game/AntizeInventory/Blueprints/Inventory/BP_InventoryComponent.BP_InventoryComponent_C|GetInventorySlots _inventoryref))
  (LocalVariables|SetLocal_StorageIndex StorageIndex)
  (LocalVariables|SetLocal_InventoryIndex InventoryIndex)
  (bind _output_get (LocalVariables|SetLocal_InvSlot (Utilities|Array|Get(acopy) (Variables|/Game/AntizeInventory/Blueprints/Inventory/BP_InventoryComponent.BP_InventoryComponent_C|GetInventorySlots (Variables|Spawn|GetInventoryRef)) (LocalVariables|GetLocal_InventoryIndex))))
  (if (> (Utilities|Struct|BreakS_InventorySlot (LocalVariables|GetLocal_InvSlot)) 0)
    (bind _returnvalue (Utilities|GetDataTableRow "/Game/AntizeInventory/Logics/Datatable/DT_Item.DT_Item" (.RowName (Utilities|Struct|BreakDataTableRowHandle (Utilities|Struct|BreakS_InventorySlot _output_get))))
      (:then
        (LocalVariables|SetLocal_InvItem _returnvalue)
        (bind _output_get_2 (LocalVariables|SetLocal_StorageSlot (Utilities|Array|Get(acopy) (Variables|Traitement|GetStorageSlots) (LocalVariables|GetLocal_StorageIndex))))
        (bind _returnvalue_2 (Utilities|GetDataTableRow "/Game/AntizeInventory/Logics/Datatable/DT_Item.DT_Item" (.RowName (Utilities|Struct|BreakDataTableRowHandle (Utilities|Struct|BreakS_InventorySlot _output_get_2))))
          (:then
            (LocalVariables|SetLocal_StorageItem _returnvalue_2)
            (if (Math|Boolean|ANDBoolean (> (Utilities|Struct|BreakS_Item (LocalVariables|GetLocal_StorageItem)) 1) (Utilities|Name|Equal(Name) (.RowName (Utilities|Struct|BreakDataTableRowHandle (Utilities|Struct|BreakS_InventorySlot (LocalVariables|GetLocal_InvSlot)))) (.RowName (Utilities|Struct|BreakDataTableRowHandle (Utilities|Struct|BreakS_InventorySlot (LocalVariables|GetLocal_StorageSlot))))) (< (Utilities|Struct|BreakS_InventorySlot (LocalVariables|GetLocal_StorageSlot)) (Utilities|Struct|BreakS_Item (LocalVariables|GetLocal_StorageItem))))
              (if (>= (- (Utilities|Struct|BreakS_Item (LocalVariables|GetLocal_StorageItem)) (Utilities|Struct|BreakS_InventorySlot (LocalVariables|GetLocal_StorageSlot))) (Utilities|Struct|BreakS_InventorySlot (LocalVariables|GetLocal_InvSlot)))
                (Utilities|Struct|SetmembersinS_InventorySlot (Utilities|Array|Get(acopy) (Variables|Traitement|GetStorageSlots) (LocalVariables|GetLocal_StorageIndex)) (+ (Utilities|Struct|BreakS_InventorySlot (LocalVariables|GetLocal_StorageSlot)) (Utilities|Struct|BreakS_InventorySlot (LocalVariables|GetLocal_InvSlot))))
                (Utilities|Array|SetArrayElem _inventoryslots (LocalVariables|GetLocal_InventoryIndex) (Utilities|Struct|MakeS_InventorySlot (Utilities|Struct|MakeDataTableRowHandle 0 "None") 0 0))
                (else
                  (Utilities|Struct|SetmembersinS_InventorySlot (Utilities|Array|Get(acopy) (Variables|Traitement|GetStorageSlots) (LocalVariables|GetLocal_StorageIndex)) (Utilities|Struct|BreakS_Item (LocalVariables|GetLocal_StorageItem)))
                  (Utilities|Struct|SetmembersinS_InventorySlot (Utilities|Array|Get(acopy) _inventoryslots (LocalVariables|GetLocal_InventoryIndex)) (- (Utilities|Struct|BreakS_InventorySlot (LocalVariables|GetLocal_InvSlot)) (- (Utilities|Struct|BreakS_Item (LocalVariables|GetLocal_InvItem)) (Utilities|Struct|BreakS_InventorySlot (LocalVariables|GetLocal_StorageSlot)))))))
              (else
                ;[1 1 1] Swap Inventory Slot and Storage Slot
                (Utilities|Array|SetArrayElem (Variables|Traitement|GetStorageSlots) (LocalVariables|GetLocal_StorageIndex) (LocalVariables|GetLocal_InvSlot))
                (Utilities|Array|SetArrayElem (Variables|/Game/AntizeInventory/Blueprints/Inventory/BP_InventoryComponent.BP_InventoryComponent_C|GetInventorySlots (Variables|Spawn|GetInventoryRef)) (LocalVariables|GetLocal_InventoryIndex) (LocalVariables|GetLocal_StorageSlot)))))
          (:RowNotFound
            ;[1 1 1] Move item from Inventory to Storage
            (Utilities|Array|SetArrayElem (Variables|Traitement|GetStorageSlots) (LocalVariables|GetLocal_StorageIndex) (LocalVariables|GetLocal_InvSlot))
            (Utilities|Array|SetArrayElem (Variables|/Game/AntizeInventory/Blueprints/Inventory/BP_InventoryComponent.BP_InventoryComponent_C|GetInventorySlots (Variables|Spawn|GetInventoryRef)) (LocalVariables|GetLocal_InventoryIndex) (Utilities|Struct|MakeS_InventorySlot (Utilities|Struct|MakeDataTableRowHandle 0 "None") 0 0))))
        ;[1 1 1] Refresh Inventory Slot and Storage Slot
        (Default|RemovePadatIndex (Variables|Spawn|GetInventoryRef) (LocalVariables|GetLocal_InventoryIndex))
        (Default|FactoriseUpdateInventorySlot (Variables|Spawn|GetInventoryRef) (LocalVariables|GetLocal_InventoryIndex))
        (Default|UpdateSlotWidgetatIndex (Variables|Spawn|GetW_StorageRef) (LocalVariables|GetLocal_StorageIndex))
        (bind _equippedweapon (Class|BPInventoryInterface|MSGGetEquippedWeapon(Message) (Variables|/Game/AntizeInventory/Blueprints/Inventory/BP_InventoryComponent.BP_InventoryComponent_C|GetCharacterRef (Variables|Spawn|GetInventoryRef))))
        (if (== (Utilities|Struct|BreakS_WeaponCharacteristics _equippedweapon) (LocalVariables|GetLocal_InventoryIndex))
          (Class|BPInventoryInterface|MSGUnequipWeapon(Message) (Variables|/Game/AntizeInventory/Blueprints/Inventory/BP_InventoryComponent.BP_InventoryComponent_C|GetCharacterRef (Variables|Spawn|GetInventoryRef)))
          (return true)
          (else
            (return true))))
      (:RowNotFound
        _)))
  (return false))

(fn CombineorSwapSlot
  (params (IndexFrom :type Integer) (IndexTo :type Integer))
  (LocalVariables|SetLocal_IndexFrom IndexFrom)
  (LocalVariables|SetLocal_IndexTo IndexTo)
  (bind _output_get (LocalVariables|SetLocal_SlotFrom (Utilities|Array|Get(acopy) (Variables|Traitement|GetStorageSlots) (LocalVariables|GetLocal_IndexFrom))))
  (bind _returnvalue (Utilities|GetDataTableRow "/Game/AntizeInventory/Logics/Datatable/DT_Item.DT_Item" (.RowName (Utilities|Struct|BreakDataTableRowHandle (Utilities|Struct|BreakS_InventorySlot _output_get))))
    (:then
      (LocalVariables|SetLocal_ItemFrom _returnvalue)
      (bind _output_get_2 (LocalVariables|SetLocal_SlotTo (Utilities|Array|Get(acopy) (Variables|Traitement|GetStorageSlots) (LocalVariables|GetLocal_IndexTo))))
      (bind _returnvalue_2 (Utilities|GetDataTableRow "/Game/AntizeInventory/Logics/Datatable/DT_Item.DT_Item" (.RowName (Utilities|Struct|BreakDataTableRowHandle (Utilities|Struct|BreakS_InventorySlot _output_get_2))))
        (:then
          (LocalVariables|SetLocal_ItemTo _returnvalue_2)
          (if (Math|Boolean|ANDBoolean (> (Utilities|Struct|BreakS_Item (LocalVariables|GetLocal_ItemTo)) 1) (Utilities|Name|Equal(Name) (.RowName (Utilities|Struct|BreakDataTableRowHandle (Utilities|Struct|BreakS_InventorySlot (LocalVariables|GetLocal_SlotFrom)))) (.RowName (Utilities|Struct|BreakDataTableRowHandle (Utilities|Struct|BreakS_InventorySlot (LocalVariables|GetLocal_SlotTo))))) (< (Utilities|Struct|BreakS_InventorySlot (LocalVariables|GetLocal_SlotTo)) (Utilities|Struct|BreakS_Item (LocalVariables|GetLocal_ItemTo))))
            (if (>= (- (Utilities|Struct|BreakS_Item (LocalVariables|GetLocal_ItemTo)) (Utilities|Struct|BreakS_InventorySlot (LocalVariables|GetLocal_SlotTo))) (Utilities|Struct|BreakS_InventorySlot (LocalVariables|GetLocal_SlotFrom)))
              (Utilities|Struct|SetmembersinS_InventorySlot (Utilities|Array|Get(acopy) (Variables|Traitement|GetStorageSlots) (LocalVariables|GetLocal_IndexTo)) (+ (Utilities|Struct|BreakS_InventorySlot (LocalVariables|GetLocal_SlotTo)) (Utilities|Struct|BreakS_InventorySlot (LocalVariables|GetLocal_SlotFrom))))
              (Utilities|Array|SetArrayElem (Variables|Traitement|GetStorageSlots) (LocalVariables|GetLocal_IndexFrom) (Utilities|Struct|MakeS_InventorySlot (Utilities|Struct|MakeDataTableRowHandle 0 "None") 0 0))
              (else
                (Utilities|Struct|SetmembersinS_InventorySlot (Utilities|Array|Get(acopy) (Variables|Traitement|GetStorageSlots) (LocalVariables|GetLocal_IndexTo)) (Utilities|Struct|BreakS_Item (LocalVariables|GetLocal_ItemTo)))
                (Utilities|Struct|SetmembersinS_InventorySlot (Utilities|Array|Get(acopy) (Variables|Traitement|GetStorageSlots) (LocalVariables|GetLocal_IndexFrom)) (- (Utilities|Struct|BreakS_InventorySlot (LocalVariables|GetLocal_SlotFrom)) (- (Utilities|Struct|BreakS_Item (LocalVariables|GetLocal_ItemTo)) (Utilities|Struct|BreakS_InventorySlot (LocalVariables|GetLocal_SlotTo)))))))
            ;[1 1 1] Refresh Storage Slots
            (Default|UpdateSlotWidgetatIndex (Variables|Spawn|GetW_StorageRef) (LocalVariables|GetLocal_IndexFrom))
            (Default|UpdateSlotWidgetatIndex (Variables|Spawn|GetW_StorageRef) (LocalVariables|GetLocal_IndexTo))
            (return true)
            (else
              (Utilities|Array|SetArrayElem (Variables|Traitement|GetStorageSlots) (LocalVariables|GetLocal_IndexFrom) (LocalVariables|GetLocal_SlotTo))
              (Utilities|Array|SetArrayElem (Variables|Traitement|GetStorageSlots) (LocalVariables|GetLocal_IndexTo) (LocalVariables|GetLocal_SlotFrom)))))
        (:RowNotFound
          (Utilities|Array|SetArrayElem (Variables|Traitement|GetStorageSlots) (LocalVariables|GetLocal_IndexFrom) (Utilities|Struct|MakeS_InventorySlot (Utilities|Struct|MakeDataTableRowHandle 0 "None") 0 0))
          (Utilities|Array|SetArrayElem (Variables|Traitement|GetStorageSlots) (LocalVariables|GetLocal_IndexTo) (LocalVariables|GetLocal_SlotFrom))))
      ;[1 1 1] Refresh Storage Slots
      (Default|UpdateSlotWidgetatIndex (Variables|Spawn|GetW_StorageRef) (LocalVariables|GetLocal_IndexFrom))
      (Default|UpdateSlotWidgetatIndex (Variables|Spawn|GetW_StorageRef) (LocalVariables|GetLocal_IndexTo))
      (return true))
    (:RowNotFound
      (return false))))

(fn SearchEmptySlot
  (bind _array_index (Utilities|Array|ForEachLoopwithBreak (Variables|Traitement|GetStorageSlots) :!label _label)
    (:LoopBody
      (if (Storage|GetIsSlotEmpty _array_index)
        (LocalVariables|SetLocal_Found? true)
        (LocalVariables|SetLocal_Index _array_index)
        (goto _label Break)))
    (:Completed
      (return (LocalVariables|GetLocal_Found?) (LocalVariables|GetLocal_Index)))))

(fn GetIsSlotEmpty
  (params (Index :type Integer))
  (bind _storageslots (Variables|Traitement|GetStorageSlots))
  (bind _output (Utilities|Array|Get(acopy) _storageslots Index))
  (bind (_item _amount) (Utilities|Struct|BreakS_InventorySlot _output))
  (Utilities|GetDataTableRow "/Game/AntizeInventory/Logics/Datatable/DT_Item.DT_Item" (.rowname _item)
    (:then
      (return (<= _amount 0)))
    (:RowNotFound
      (return true))))

(fn UpdateVariables
  (params (InventoryRef :type BP%20Inventory%20Component%20Object%20Reference))
  (bind _output_get (Variables|Spawn|SetInventoryRef InventoryRef))
  (Variables|Spawn|SetW_StorageRef (Variables|/Game/AntizeInventory/Widgets/Inventory/W_Inventory.W_Inventory_C|GetW_Storage (Variables|/Game/AntizeInventory/Blueprints/Inventory/BP_InventoryComponent.BP_InventoryComponent_C|GetW_InventoryRef _output_get)))
  (return))

(fn LoadStorageSlots
  (bind (_slotname _userindex) (CallFunction|GetSlotNameUserIndex))
  (bind _storagename (Variables|Spawn|Save|GetStorageName))
  (bind _returnvalue (Math|Conversions|ToInteger(Byte) _storagename))
  (bind _slotsave (CallFunction|LoadSlots _slotname _userindex))
  (bind _output_get (Variables|Spawn|Save|SetSlotSave _slotsave))
  (Utilities|IsValid _output_get
    (:Is%20Valid
      (if (Variables|/Game/AntizeInventory/Blueprints/SaveGame/BP_SaveInventory.BP_SaveInventory_C|GetSaved? _output_get)
        (if (Utilities|Array|IsValidIndex (Variables|/Game/AntizeInventory/Blueprints/SaveGame/BP_SaveInventory.BP_SaveInventory_C|GetSave_StorageSlots (Variables|Spawn|Save|GetSlotSave)) _returnvalue)
          (Variables|Traitement|SetStorageSlots (Utilities|Struct|BreakS_SaveStorage (Utilities|Array|Get(acopy) (Variables|/Game/AntizeInventory/Blueprints/SaveGame/BP_SaveInventory.BP_SaveInventory_C|GetSave_StorageSlots (Variables|Spawn|Save|GetSlotSave)) _returnvalue))))))
    (:Is%20Not%20Valid
      _))
  (return))

(fn DoSaveStorageSlots
  (params (SaveRef :type BP%20Save%20Inventory%20Object%20Reference))
  (bind _output_get (LocalVariables|SetLocal_SaveRef SaveRef))
  (Utilities|Array|SetArrayElem (Variables|/Game/AntizeInventory/Blueprints/SaveGame/BP_SaveInventory.BP_SaveInventory_C|GetSave_StorageSlots _output_get) (Math|Conversions|ToInteger(Byte) (Variables|Spawn|Save|GetStorageName)) (Utilities|Struct|MakeS_SaveStorage (Variables|Traitement|GetStorageSlots)) true)
  (return))