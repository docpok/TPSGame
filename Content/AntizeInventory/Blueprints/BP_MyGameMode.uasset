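; Game mode for the Antize inventory system that restores saved world loot and records destroyed loot, acting on the server only.
; Shortly after BeginPlay it prints warnings for duplicate storage, loot and door names, then loads the save slot.
; Saveable loot actors are matched to saved entries by display name, then updated or destroyed if depleted.
; Message functions add and return destroyed loot names; the weapon, inventory and stats getters are stubs.
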(event EventBeginPlay
  ;[1 1 1] Constructor
  (Networking|SwitchHasAuthority
    (:Authority
      (Utilities|FlowControl|Delay 0.2)
      (CallFunction|CheckforDuplicateName)
      (CallFunction|LoadWorldLoot))))

(event EventMSGAddDestroyedLoot
  (params (LootName :type String))
  ;[1 1 1] Add loot in destroyed array
  (Networking|SwitchHasAuthority
    (:Authority
      (CallFunction|AddDestroyedLoot LootName))))

(fn ConstructionScript)

(fn CheckforDuplicateName
  (bind _local_doorname (LocalVariables|GetLocal_DoorName))
  (bind _local_lootname (LocalVariables|GetLocal_LootName))
  ;[1 1 1] Print a warning message if duplicated save setting or name is found
  (bind _outactors (Actor|GetAllActorsOfClass "/Game/AntizeInventory/Blueprints/Storage/BP_MasterStorage.BP_MasterStorage_C"))
  (for _array_element _outactors
    (if (Utilities|Enum|NotEqual(Enum) (Variables|/Game/AntizeInventory/Blueprints/Storage/BP_MasterStorage.BP_MasterStorage_C|GetStorageName _array_element) "NewEnumerator0")
      (if (Utilities|Array|ContainsItem (LocalVariables|GetLocal_Name) (Variables|/Game/AntizeInventory/Blueprints/Storage/BP_MasterStorage.BP_MasterStorage_C|GetStorageName _array_element))
        (Development|PrintString (Utilities|String|Append "Warning : Duplicate Storage Name - " (Utilities|String|EnumtoString (Variables|/Game/AntizeInventory/Blueprints/Storage/BP_MasterStorage.BP_MasterStorage_C|GetStorageName _array_element)) " -> " (Utilities|GetDisplayName _array_element) " (E_SaveName)") true true "(R=1.000000,G=0.677696,B=0.000000,A=1.000000)" 1e+01)
        (else
          (Utilities|Array|Add (LocalVariables|GetLocal_Name) (Variables|/Game/AntizeInventory/Blueprints/Storage/BP_MasterStorage.BP_MasterStorage_C|GetStorageName _array_element))))))
  (bind _outactors_2 (Actor|GetAllActorsOfClass "/Game/AntizeInventory/Blueprints/Inventory/BP_Loot.BP_Loot_C"))
  (for _array_element_2 _outactors_2
    (if (Utilities|Array|ContainsItem _local_lootname (Utilities|GetDisplayName _array_element_2))
      (Development|PrintString (Utilities|String|Append "Warning : Duplicate Loot Name - " " -> " (Utilities|GetDisplayName _array_element_2)) true true "(R=1.000000,G=0.677696,B=0.000000,A=1.000000)" 1e+01)
      (else
        (Utilities|Array|Add _local_lootname (Utilities|GetDisplayName _array_element_2)))))
  (bind _outactors_3 (Actor|GetAllActorsOfClass "/Game/AntizeInventory/Blueprints/Other/BP_Door.BP_Door_C"))
  (for _array_element_3 _outactors_3
    (if (Utilities|Array|ContainsItem _local_doorname (Utilities|GetDisplayName _array_element_3))
      (Development|PrintString (Utilities|String|Append "Warning : Duplicate Door Name - " " -> " (Utilities|GetDisplayName _array_element_3)) true true "(R=1.000000,G=0.677696,B=0.000000,A=1.000000)" 1e+01)
      (else
        (Utilities|Array|Add _local_doorname (Utilities|GetDisplayName _array_element_3))))))

(fn LoadWorldLoot
  (bind (_slotname _userindex) (CallFunction|GetSlotNameUserIndex))
  ;[1 1 1] If loot can be modified by saving, apply loaded data
  (bind _slotsave (CallFunction|LoadSlots _slotname _userindex))
  (if (Variables|/Game/AntizeInventory/Blueprints/SaveGame/BP_SaveInventory.BP_SaveInventory_C|GetSaved? _slotsave)
    (bind _output_get (LocalVariables|SetLocal_Save _slotsave))
    (for _array_element (Variables|/Game/AntizeInventory/Blueprints/SaveGame/BP_SaveInventory.BP_SaveInventory_C|GetSave_Loot _output_get)
      (Utilities|Array|Add (LocalVariables|GetLocal_LootName) (Utilities|Struct|BreakS_SaveLoot _array_element)))
    (if (> (Utilities|Array|Length (LocalVariables|GetLocal_LootName)) 0)
      (bind _outactors (Actor|GetAllActorsOfClass "/Game/AntizeInventory/Blueprints/Inventory/BP_Loot.BP_Loot_C"))
      (for _array_element_2 _outactors
        (if (not (Variables|/Game/AntizeInventory/Blueprints/Inventory/BP_Loot.BP_Loot_C|GetIgnoreSaving? _array_element_2))
          (bind _output_get_2 (LocalVariables|SetLocal_FindIndex (Utilities|Array|FindItem (LocalVariables|GetLocal_LootName) (Utilities|GetDisplayName _array_element_2))))
          (if (>= _output_get_2 0)
            (if (<= (Utilities|Struct|BreakS_InventorySlot (Utilities|Struct|BreakS_SaveLoot (Utilities|Array|Get(acopy) (Variables|/Game/AntizeInventory/Blueprints/SaveGame/BP_SaveInventory.BP_SaveInventory_C|GetSave_Loot (LocalVariables|GetLocal_Save)) (LocalVariables|GetLocal_FindIndex)))) 0)
              (Actor|DestroyActor _array_element_2)
              (else
                (Variables|/Game/AntizeInventory/Blueprints/Inventory/BP_Loot.BP_Loot_C|SetItemOnLoot _array_element_2 (Utilities|Struct|BreakS_SaveLoot (Utilities|Array|Get(acopy) (Variables|/Game/AntizeInventory/Blueprints/SaveGame/BP_SaveInventory.BP_SaveInventory_C|GetSave_Loot (LocalVariables|GetLocal_Save)) (LocalVariables|GetLocal_FindIndex)))))))))
      (return)
      (else
        (return)))
    (else
      (return))))

(fn AddDestroyedLoot
  (params (LootName :type String))
  (if (Utilities|Array|ContainsItem (Variables|Default|GetLootDestroyed) LootName)
    _
    (else
      (Utilities|Array|Add (Variables|Default|GetLootDestroyed) LootName)))
  (return))

(fn MSGGetDestroyedLoot
  (return (Variables|Default|GetLootDestroyed)))

(fn MSGGetEquippedWeapon
  (return ""))

(fn MSGGetInventory
  (return 0))

(fn MSGGetStats
  (return 0.0 0.0 0.0))