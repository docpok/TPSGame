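; AntizeKit game mode acting as the server-side hub for players, teams, pings and saved world loot.
; Login and logout maintain a connected-player list with unique IDs, used to relay system messages, answer player lookups and route pings by team.
; Joining a team clears old pings, assigns a free slot as color ID and refreshes team markers.
; BeginPlay warns of duplicate save names, then applies saved amounts to or destroys loot actors.
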(event Custom|SendsSystemMessageToPlayers
  (params (Message :type Text))
  ;[1 1 1] Sends a system message to players
  (Networking|SwitchHasAuthority
    (:Authority
      (for _array_element (Variables|General|GetConnectedPlayers)
        (Utilities|IsValid _array_element
          (:Is%20Valid
            (Class|BPAntizeChatInterface|MSGNewMessage(Message) _array_element true "NewEnumerator5" -1 -1 "" Message "NewEnumerator0")))))))

(event Custom|ChangeDifficulty
  (params (NewDifficulty :type E_Difficulty%20Enum :default "NewEnumerator0"))
  ;[1 1 1] Difficulty changed (Exemple)
  (Variables|MenuSystem|SetCurrentDifficulty NewDifficulty))

(event EventBeginPlay
  ;[1 1 1] Constructor
  (Networking|SwitchHasAuthority
    (:Authority
      (Utilities|FlowControl|Delay 0.2)
      (InventorySystem|CheckforDuplicateName)
      (InventorySystem|LoadWorldLoot))))

(event EventPostLogin
  (params (NewPlayer :type Player%20Controller%20Object%20Reference))
  (bind _uniqueplayerid (Variables|General|GetUniquePlayerID))
  ;[1 1 1] On new player - Add player to PlayersConnected array
  (Networking|SwitchHasAuthority
    (:Authority
      (Utilities|IsValid NewPlayer
        (:Is%20Valid
          (Utilities|Array|AddUnique (Variables|General|GetConnectedPlayers) NewPlayer)
          (Class|BPAntizeChatInterface|MSGSetPlayerID(Message) NewPlayer _uniqueplayerid)
          (Math|Integer|IncrementInt _uniqueplayerid))))))

(event EventOnLogout
  (params (ExitingController :type Controller%20Object%20Reference))
  ;[1 1 1] On player left - Remove player from PlayersConnected array
  (Networking|SwitchHasAuthority
    (:Authority
      (Utilities|Array|RemoveItem (Variables|General|GetConnectedPlayers) ExitingController))))

(event EventMSGAddDestroyedLoot
  (params (LootName :type String))
  ;[1 1 1] Add loot in destroyed array
  (Networking|SwitchHasAuthority
    (:Authority
      (InventorySystem|AddDestroyedLoot LootName))))

(event Custom|RemoveSystemPing
  ;[0.1448 1 0.2029] Secure remove all ping system
  (Networking|SwitchHasAuthority
    (:Authority
      (if (> (Utilities|Array|Length (Variables|PingSystem|GetActualRandomPing)) 0) :!label _label
        (Utilities|FlowControl|Delay 0.01)
        (for _array_element (Variables|General|GetConnectedPlayers)
          (Class|BPAntizePingInterface|MSGRemovePing(Message) _array_element (Utilities|Array|Get(acopy) (Variables|PingSystem|GetActualRandomPing)) -1 false))
        (Utilities|Array|RemoveIndex (Variables|PingSystem|GetActualRandomPing))
        (goto _label)))))

(event EventMSGPingonPing
  (params (Add? :type Boolean) (PingOwnerID :type Integer) (TeamID :type Integer) (ColorID :type Integer))
  ;[0.1448 1 0.2029] (From Controller) PingOnPing receveid
  (Networking|SwitchHasAuthority
    (:Authority
      (if (>= TeamID 0)
        (for _array_element (Variables|General|GetConnectedPlayers)
          (Utilities|IsValid _array_element
            (:Is%20Valid
              (bind _teamid (Class|BPAntizeChatInterface|MSGGetTeamID(Message) _array_element))
              (if (== _teamid TeamID)
                (Class|BPAntizePingInterface|MSGPingonPing(Message) _array_element Add? PingOwnerID TeamID ColorID)))))))))

(event EventMSGAddPing
  (params (Location :type Vector :default "0, 0, 0") (Type :type E_PingType%20Enum :default "NewEnumerator1") (ActorHit :type Actor%20Object%20Reference) (OwnerID :type Integer) (TeamID :type Integer) (ColorID :type Integer) (BySystem? :type Boolean))
  ;[0.1448 1 0.2029] (From Controller) New ping receveid (Does't send if TeamID is less than 0 (Not system) but the player can ping for himself)
  (Networking|SwitchHasAuthority
    (:Authority
      (bind _array_element (Utilities|Array|ForEachLoopwithBreak (Variables|General|GetConnectedPlayers) :!label _label)
        (:LoopBody
          (Utilities|IsValid _array_element
            (:Is%20Valid
              (if (>= TeamID 0)
                (bind _teamid (Class|BPAntizeChatInterface|MSGGetTeamID(Message) _array_element))
                (if (== _teamid TeamID)
                  (Class|BPAntizePingInterface|MSGAddPing(Message) _array_element Location Type ActorHit OwnerID TeamID ColorID BySystem? :!label _label_2))
                (elif BySystem?
                  (goto _label_2)
                  (else
                    (bind _playerid (Class|BPAntizeChatInterface|MSGGetPlayerID(Message) _array_element))
                    (if (== _playerid OwnerID)
                      (Utilities|FlowControl|Sequence
                        (:then_0
                          (goto _label_2))
                        (:then_1
                          (goto _label Break))))))))))))))

(event EventTick
  (params (DeltaSeconds :type Float%20%28single-precision%29))
  ;[1 0 0] Only for test, must be deleted
)

(event EventMSGRemovePing
  (params (OwnerID :type Integer) (ColorID :type Integer) (PlaySound? :type Boolean))
  ;[0.1448 1 0.2029] (From Controller) Remove ping receveid
  (Networking|SwitchHasAuthority
    (:Authority
      (for _array_element (Variables|General|GetConnectedPlayers)
        (Utilities|IsValid _array_element
          (:Is%20Valid
            (Class|BPAntizePingInterface|MSGRemovePing(Message) _array_element OwnerID ColorID PlaySound?)))))))

(event EventMSGJoinTeam
  (params (PlayerRef :type Player%20Controller%20Object%20Reference) (FromTeamID :type Integer) (ToTeamID :type Integer))
  ;[0.1448 1 0.2029] (From Controller) Join Team receveid
  (Networking|SwitchHasAuthority
    (:Authority
      (PingSystem|JoinTeam PlayerRef FromTeamID ToTeamID))))

(fn ConstructionScript)

(fn ResetPlayerID
  (bind _local_attempt (LocalVariables|GetLocal_Attempt))
  (bind _local_index (LocalVariables|GetLocal_Index))
  (bind _returnvalue (Game|GetPlayerController _local_index))
  (Networking|SwitchHasAuthority
    (:Authority
      (LocalVariables|SetLocal_Continue? true)
      (Variables|General|SetUniquePlayerID 0)
      (while (LocalVariables|GetLocal_Continue?)
        (Utilities|IsValid _returnvalue
          (:Is%20Valid
            (Utilities|Array|Add (LocalVariables|GetLocal_Controller) _returnvalue)
            (Class|BPAntizeChatInterface|MSGSetPlayerID(Message) _returnvalue (Variables|General|GetUniquePlayerID))
            (Math|Integer|IncrementInt (LocalVariables|GetLocal_Index)
              (:%20%20
                (Math|Integer|IncrementInt (Variables|General|GetUniquePlayerID)))))
          (:Is%20Not%20Valid
            ;[1 1 1] Be sure to try more index if a player is not valid
            (if (>= _local_attempt 5)
              (LocalVariables|SetLocal_Continue? false)
              (else
                (Math|Integer|IncrementInt _local_attempt
                  (:%20%20
                    (Math|Integer|IncrementInt (LocalVariables|GetLocal_Index)))))))))
      (Variables|General|SetConnectedPlayers (LocalVariables|GetLocal_Controller))
      (return))))

(fn CheckforDuplicateName
  (bind _local_doorname (LocalVariables|GetLocal_DoorName))
  (bind _local_lootname (LocalVariables|GetLocal_LootName))
  ;[1 1 1] Print a warning message if duplicated save setting or name is found
  (bind _outactors (Actor|GetAllActorsOfClass "/Game/AntizeKitSystem/AntizeSystems/InventorySystem/Blueprints/Storage/BP_MasterStorage.BP_MasterStorage_C"))
  (for _array_element _outactors
    (if (Utilities|Enum|NotEqual(Enum) (Variables|/Game/AntizeKitSystem/AntizeSystems/InventorySystem/Blueprints/Storage/BP_MasterStorage.BP_MasterStorage_C|GetStorageName _array_element) "NewEnumerator0")
      (if (Utilities|Array|ContainsItem (LocalVariables|GetLocal_Name) (Variables|/Game/AntizeKitSystem/AntizeSystems/InventorySystem/Blueprints/Storage/BP_MasterStorage.BP_MasterStorage_C|GetStorageName _array_element))
        (Development|PrintString (Utilities|String|Append "Warning : Duplicate Storage Name - " (Utilities|String|EnumtoString (Variables|/Game/AntizeKitSystem/AntizeSystems/InventorySystem/Blueprints/Storage/BP_MasterStorage.BP_MasterStorage_C|GetStorageName _array_element)) " -> " (Utilities|GetDisplayName _array_element) " (E_SaveName)") true true "(R=1.000000,G=0.677696,B=0.000000,A=1.000000)" 1e+01)
        (else
          (Utilities|Array|Add (LocalVariables|GetLocal_Name) (Variables|/Game/AntizeKitSystem/AntizeSystems/InventorySystem/Blueprints/Storage/BP_MasterStorage.BP_MasterStorage_C|GetStorageName _array_element))))))
  (bind _outactors_2 (Actor|GetAllActorsOfClass "/Game/AntizeKitSystem/AntizeSystems/InventorySystem/Blueprints/Inventory/BP_Loot.BP_Loot_C"))
  (for _array_element_2 _outactors_2
    (if (Utilities|Array|ContainsItem _local_lootname (Utilities|GetDisplayName _array_element_2))
      (Development|PrintString (Utilities|String|Append "Warning : Duplicate Loot Name - " " -> " (Utilities|GetDisplayName _array_element_2)) true true "(R=1.000000,G=0.677696,B=0.000000,A=1.000000)" 1e+01)
      (else
        (Utilities|Array|Add _local_lootname (Utilities|GetDisplayName _array_element_2)))))
  (bind _outactors_3 (Actor|GetAllActorsOfClass "/Game/AntizeKitSystem/AntizeSystems/InventorySystem/Blueprints/Other/BP_Door.BP_Door_C"))
  (for _array_element_3 _outactors_3
    (if (Utilities|Array|ContainsItem _local_doorname (Utilities|GetDisplayName _array_element_3))
      (Development|PrintString (Utilities|String|Append "Warning : Duplicate Door Name - " " -> " (Utilities|GetDisplayName _array_element_3)) true true "(R=1.000000,G=0.677696,B=0.000000,A=1.000000)" 1e+01)
      (else
        (Utilities|Array|Add _local_doorname (Utilities|GetDisplayName _array_element_3))))))

(fn LoadWorldLoot
  ;[1 1 1] If loot can be modified by saving, apply loaded data
  (bind _saveref (Class|BPAntizeKitInterface|MSGGetSave(Message) (Game|GetGameInstance)))
  (Utilities|IsValid _saveref
    (:Is%20Valid
      (if (Variables|/Game/AntizeKitSystem/AntizeSystems/InventorySystem/Blueprints/SaveGame/BP_SaveInventory.BP_SaveInventory_C|GetSaved? _saveref)
        (bind _output_get (LocalVariables|SetLocal_Save _saveref))
        (for _array_element (Variables|/Game/AntizeKitSystem/AntizeSystems/InventorySystem/Blueprints/SaveGame/BP_SaveInventory.BP_SaveInventory_C|GetSave_Loot _output_get)
          (Utilities|Array|Add (LocalVariables|GetLocal_LootName) (Utilities|Struct|BreakS_SaveLoot _array_element)))
        (if (> (Utilities|Array|Length (LocalVariables|GetLocal_LootName)) 0)
          (bind _outactors (Actor|GetAllActorsOfClass "/Game/AntizeKitSystem/AntizeSystems/InventorySystem/Blueprints/Inventory/BP_Loot.BP_Loot_C"))
          (for _array_element_2 _outactors
            (if (not (Variables|/Game/AntizeKitSystem/AntizeSystems/InventorySystem/Blueprints/Inventory/BP_Loot.BP_Loot_C|GetIgnoreSaving? _array_element_2))
              (bind _output_get_2 (LocalVariables|SetLocal_FindIndex (Utilities|Array|FindItem (LocalVariables|GetLocal_LootName) (Utilities|GetDisplayName _array_element_2))))
              (if (>= _output_get_2 0)
                (if (<= (Utilities|Struct|BreakS_InventorySlot (Utilities|Struct|BreakS_SaveLoot (Utilities|Array|Get(acopy) (Variables|/Game/AntizeKitSystem/AntizeSystems/InventorySystem/Blueprints/SaveGame/BP_SaveInventory.BP_SaveInventory_C|GetSave_Loot (LocalVariables|GetLocal_Save)) (LocalVariables|GetLocal_FindIndex)))) 0)
                  (Actor|DestroyActor _array_element_2)
                  (else
                    (Variables|/Game/AntizeKitSystem/AntizeSystems/InventorySystem/Blueprints/Inventory/BP_Loot.BP_Loot_C|SetItemOnLoot _array_element_2 (Utilities|Struct|BreakS_SaveLoot (Utilities|Array|Get(acopy) (Variables|/Game/AntizeKitSystem/AntizeSystems/InventorySystem/Blueprints/SaveGame/BP_SaveInventory.BP_SaveInventory_C|GetSave_Loot (LocalVariables|GetLocal_Save)) (LocalVariables|GetLocal_FindIndex)))))))))
          (return)
          (else
            (return)))
        (else
          _)))
    (:Is%20Not%20Valid
      _))
  (return))

(fn AddDestroyedLoot
  (params (LootName :type String%20%28by%20ref%29))
  (if (Utilities|Array|ContainsItem (Variables|InventorySystem|GetLootDestroyed) LootName)
    _
    (else
      (Utilities|Array|Add (Variables|InventorySystem|GetLootDestroyed) LootName)))
  (return))

(fn JoinTeam
  (params (PlayerRef :type Player%20Controller%20Object%20Reference) (FromTeamID :type Integer) (ToTeamID :type Integer))
  (Networking|SwitchHasAuthority
    (:Authority
      (Utilities|IsValid PlayerRef
        (:Is%20Valid
          (LocalVariables|SetLocal_PlayerRef PlayerRef)
          (LocalVariables|SetLocal_FromTeamID FromTeamID)
          (LocalVariables|SetLocal_ToTeamID ToTeamID)
          ;[1 1 1] Don't continue if already in the Team
          (bind _teamid (Class|BPAntizeChatInterface|MSGGetTeamID(Message) (LocalVariables|GetLocal_PlayerRef)))
          (if (and (!= _teamid (LocalVariables|GetLocal_ToTeamID)) (!= (LocalVariables|GetLocal_FromTeamID) (LocalVariables|GetLocal_ToTeamID)))
            (bind _colorid (Class|BPAntizeChatInterface|MSGGetTeamID(Message) (LocalVariables|GetLocal_PlayerRef)))
            (LocalVariables|SetLocal_TempColorID _colorid)
            (bind _playersref (PingSystem|CleanandGetPlayerinTeam (LocalVariables|GetLocal_PlayerRef) (LocalVariables|GetLocal_FromTeamID)))
            (bind _output_get (LocalVariables|SetLocal_TempFromPlayers _playersref))
            ;[1 1 1] Remove all team pings on client
            (for _array_element _output_get
              (bind _playerid (Class|BPAntizeChatInterface|MSGGetPlayerID(Message) _array_element))
              (Class|BPAntizePingInterface|MSGRemovePing(Message) (LocalVariables|GetLocal_PlayerRef) _playerid -1 false))
            ;[1 1 1] Remove all pings of the player
            (bind _playerid_2 (Class|BPAntizeChatInterface|MSGGetPlayerID(Message) (LocalVariables|GetLocal_PlayerRef)))
            (CallFunction|MSGRemovePing _playerid_2 (LocalVariables|GetLocal_TempColorID) false)
            ;[1 1 1] Remove all team markers of the player
            (PingSystem|RefreshTeamMarker (LocalVariables|GetLocal_TempFromPlayers))
            ;[1 1 1] Remove all team markers on client
            (Class|BPAntizePingInterface|MSGRefreshTeamMarker(Message) (LocalVariables|GetLocal_PlayerRef) true (Utilities|Array|MakeArray ""))
            (if (Utilities|Array|IsValidIndex (Variables|PingSystem|GetAllTeam) (LocalVariables|GetLocal_ToTeamID))
              (bind _playersref_2 (PingSystem|CleanandGetPlayerinTeam (LocalVariables|GetLocal_PlayerRef) (LocalVariables|GetLocal_ToTeamID)))
              (LocalVariables|SetLocal_TempToPlayers _playersref_2)
              ;[1 1 1] Search a free key in the team
              (bind _index (Utilities|FlowControl|ForLoopwithBreak 0 (Variables|PingSystem|GetArrayTeamMaxSize) :!label _label)
                (:LoopBody
                  (bind _output_get_2 (LocalVariables|SetLocal_KeyFound _index))
                  (if (not (.ReturnValue (Utilities|Map|Find (Utilities|Struct|BreakS_Team (Utilities|Array|Get(acopy) (Variables|PingSystem|GetAllTeam) (LocalVariables|GetLocal_ToTeamID))) _output_get_2)))
                    (LocalVariables|SetLocal_KeyFound? true)
                    (goto _label Break)))
                (:Completed
                  ;[1 1 1] If free key is found add the player in the team
                  (if (LocalVariables|GetLocal_KeyFound?)
                    (Utilities|Map|Add (Utilities|Struct|BreakS_Team (Utilities|Array|Get(acopy) (Variables|PingSystem|GetAllTeam) (LocalVariables|GetLocal_ToTeamID))) (LocalVariables|GetLocal_KeyFound) (LocalVariables|GetLocal_PlayerRef))
                    (Class|BPAntizeChatInterface|MSGSetTeamID(Message) (LocalVariables|GetLocal_PlayerRef) (LocalVariables|GetLocal_ToTeamID) (LocalVariables|GetLocal_KeyFound))
                    (Utilities|Array|AddUnique (LocalVariables|GetLocal_TempToPlayers) (LocalVariables|GetLocal_PlayerRef))
                    ;;[1 1 1] Refresh team marker (Client and player team)
                    (PingSystem|RefreshTeamMarker (LocalVariables|GetLocal_TempToPlayers))
                    (return)
                    (else
                      (Class|BPAntizeChatInterface|MSGSetTeamID(Message) (LocalVariables|GetLocal_PlayerRef) -1)
                      (Development|PrintString "No empty slot found" true true "(R=1.000000,G=0.000000,B=0.000000,A=1.000000)" 1e+01)
                      (return)))))
              (else
                ;[1 1 1] Create a new row (If index is valid)
                (if (>= (LocalVariables|GetLocal_ToTeamID) 0)
                  (Utilities|Array|SetArrayElem (Variables|PingSystem|GetAllTeam) (LocalVariables|GetLocal_ToTeamID) (Utilities|Struct|MakeS_Team (Utilities|Map|MakeMap 0 (LocalVariables|GetLocal_PlayerRef))) true))
                (Class|BPAntizeChatInterface|MSGSetTeamID(Message) (LocalVariables|GetLocal_PlayerRef) (LocalVariables|GetLocal_ToTeamID))
                (return)))
            (else
              (return))))
        (:Is%20Not%20Valid
          (return))))))

(fn CleanandGetPlayerinTeam
  (params (IgnorePlayerRef :type Player%20Controller%20Object%20Reference) (TeamID :type Integer))
  ;[1 1 1] Clean TeamID row
  (LocalVariables|SetLocal_IgnorePlayerRef IgnorePlayerRef)
  (bind _output_get (LocalVariables|SetLocal_TeamID TeamID))
  (if (>= _output_get 0)
    (bind _keys (Utilities|Map|Keys (Utilities|Struct|BreakS_Team (Utilities|Array|Get(acopy) (Variables|PingSystem|GetAllTeam) (LocalVariables|GetLocal_TeamID)))))
    (for _array_element _keys
      (bind _output_get_2 (LocalVariables|SetLocal_Key _array_element))
      (Utilities|IsValid (.Value (Utilities|Map|Find (Utilities|Struct|BreakS_Team (Utilities|Array|Get(acopy) (Variables|PingSystem|GetAllTeam) (LocalVariables|GetLocal_TeamID))) _output_get_2))
        (:Is%20Valid
          (bind _teamid (Class|BPAntizeChatInterface|MSGGetTeamID(Message) (.Value (Utilities|Map|Find (Utilities|Struct|BreakS_Team (Utilities|Array|Get(acopy) (Variables|PingSystem|GetAllTeam) (LocalVariables|GetLocal_TeamID))) _output_get_2))))
          (if (== _teamid (LocalVariables|GetLocal_TeamID))
            (Utilities|IsValid (LocalVariables|GetLocal_IgnorePlayerRef)
              (:Is%20Valid
                (if (!= (LocalVariables|GetLocal_IgnorePlayerRef) (.Value (Utilities|Map|Find (Utilities|Struct|BreakS_Team (Utilities|Array|Get(acopy) (Variables|PingSystem|GetAllTeam) (LocalVariables|GetLocal_TeamID))) _output_get_2)))
                  (Utilities|Array|AddUnique (LocalVariables|GetLocal_PlayersRef) (.Value (Utilities|Map|Find (Utilities|Struct|BreakS_Team (Utilities|Array|Get(acopy) (Variables|PingSystem|GetAllTeam) (LocalVariables|GetLocal_TeamID))) _output_get_2)) :!label _label)
                  (else
                    (Utilities|Map|Remove (Utilities|Struct|BreakS_Team (Utilities|Array|Get(acopy) (Variables|PingSystem|GetAllTeam) (LocalVariables|GetLocal_TeamID))) (LocalVariables|GetLocal_Key) :!label _label_2))))
              (:Is%20Not%20Valid
                (goto _label)))
            (else
              (goto _label_2))))
        (:Is%20Not%20Valid
          (goto _label_2))))
    (return (LocalVariables|GetLocal_PlayersRef))
    (else
      (return 0))))

(fn RefreshTeamMarker
  (params (PlayersRef :type Array%20of%20Player%20Controller%20Object%20References))
  (bind _local_ignoreplayerref (LocalVariables|GetLocal_IgnorePlayerRef))
  ;[1 1 1] Create the TeamMarker array, on the server to get the correct ID
  (for _array_element PlayersRef
    (Utilities|IsValid _array_element
      (:Is%20Valid
        (Utilities|IsValid (Pawn|GetControlledPawn _array_element)
          (:Is%20Valid
            (Utilities|IsValid _local_ignoreplayerref
              (:Is%20Valid
                (if (not (== _local_ignoreplayerref _array_element))
                  (bind (_teamid _colorid) (Class|BPAntizeChatInterface|MSGGetTeamID(Message) (Pawn|GetControlledPawn _array_element) :!label _label))
                  (Utilities|Array|Add (LocalVariables|GetLocalTeamMarker) (Utilities|Struct|MakeS_TeamMarker (Pawn|GetControlledPawn _array_element) _teamid _colorid))))
              (:Is%20Not%20Valid
                (goto _label))))
          (:Is%20Not%20Valid
            ;;[1 1 1] Remove if player is not spawned
            (Class|BPAntizePingInterface|MSGRefreshTeamMarker(Message) _array_element true (Utilities|Array|MakeArray "")))))))
  ;[1 1 1] Refresh team marker on client
  (for _array_element_2 0
    (Class|BPAntizePingInterface|MSGRefreshTeamMarker(Message) _array_element_2 false (LocalVariables|GetLocalTeamMarker)))
  (return))

(fn GetSystemID
  (bind _returnvalue (Math|Random|RandomIntegerinRange 500 999999999))
  (LocalVariables|SetLocal_SystemID _returnvalue :!label _label)
  (if (Utilities|Array|ContainsItem (Variables|PingSystem|GetActualRandomPing) _returnvalue)
    (bind _result (Math|Integer|IncrementInt (LocalVariables|GetLocal_Attempt))
      (:%20%20
        (if (< _result 500)
          (goto _label)
          (else
            (return (Math|Random|RandomIntegerinRange 500 999999999))))))
    (else
      (Utilities|Array|Add (Variables|PingSystem|GetActualRandomPing) (LocalVariables|GetLocal_SystemID))
      (return (LocalVariables|GetLocal_SystemID)))))

(fn MSGGetActorType
  (return "NewEnumerator0"))

(fn MSGGetConnectedPlayers
  (return (Variables|General|GetConnectedPlayers)))

(fn MSGGetDestroyedLoot
  (return 0))

(fn MSGGetEquippedWeapon
  (return ""))

(fn MSGGetInventory
  (return 0))

(fn MSGGetPingTexture
  (return 0))

(fn MSGGetPlayerID
  (return 0))

(fn MSGGetPlayerIDfromUsername
  (params (Username :type Text))
  (bind _array_element (Utilities|Array|ForEachLoopwithBreak (Variables|General|GetConnectedPlayers) :!label _label)
    (:LoopBody
      (bind (_success_ _username) (Class|BPAntizeChatInterface|MSGGetUsername(Message) _array_element))
      (if _success_
        (if (Utilities|Enum|Equal(Enum) _username Username)
          (bind _playerid (Class|BPAntizeChatInterface|MSGGetPlayerID(Message) _array_element))
          (LocalVariables|SetLocal_PlayerID _playerid)
          (goto _label Break))))
    (:Completed
      (return (LocalVariables|GetLocal_PlayerID)))))

(fn MSGGetStats
  (return 0.0 0.0 0.0))

(fn MSGGetTeamID
  (return 0 0))

(fn MSGGetUsername
  (return false ""))

(fn MSGRequestPrivateMessage
  (params (Request :type E_PrivateMessage%20Enum :default "NewEnumerator1") (ToPlayerID :type Integer) (Username :type Text) (Message :type Text))
  (if (>= ToPlayerID 0)
    (switch Utilities|FlowControl|Switch|SwitchonE_PrivateMessage Request
      (:NewEnumerator1
        (return (LocalVariables|GetLocal_Online?)))
      (:NewEnumerator3
        (return (LocalVariables|GetLocal_Online?)))
      (:NewEnumerator0
        (bind _array_element (Utilities|Array|ForEachLoopwithBreak (Variables|General|GetConnectedPlayers) :!label _label)
          (:LoopBody
            (bind _playerid (Class|BPAntizeChatInterface|MSGGetPlayerID(Message) _array_element))
            (if (== _playerid ToPlayerID)
              (LocalVariables|SetLocal_Online? true)
              (goto _label Break)))
          (:Completed
            (return (LocalVariables|GetLocal_Online?)))))
      (:NewEnumerator4
        (return (LocalVariables|GetLocal_Online?))))
    (else
      (return (LocalVariables|GetLocal_Online?)))))