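; BP_Save is a save-point interactable in the inventory system that shows a "Press F to save" prompt.
; On BeginPlay it sets the W_Interact widget text, then MSGInteraction shows or hides the widget by radius state and updates the displayed key.
; The interface getters for loot, equipped weapon, inventory and stats are empty stubs, and no save logic appears in this Blueprint.
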(event EventBeginPlay
  ;[1 1 1] Set interact text
  (bind _asw_interact (Utilities|Casting|CastToW_Interact (UserInterface|GetUserWidgetObject (Variables|Default|GetWidget))))
  (Rendering|Components|TextRender|SetText (Variables|/Game/AntizeKitSystem/AntizeSystems/InventorySystem/Widgets/W_Interact.W_Interact_C|GetTextBlock_Name _asw_interact) "Press F to save"))

(event EventMSGInteraction
  (params (Interaction :type E_Interaction%20Enum :default "NewEnumerator0") (Amount :type Integer) (FromActor :type Actor%20Object%20Reference) (Key :type Text))
  (bind _widget (Variables|Default|GetWidget))
  ;[1 1 1] Show/Hide Interact text
  (switch Utilities|FlowControl|Switch|SwitchonE_Interaction Interaction
    (:NewEnumerator0
      (Rendering|SetVisibility _widget true false)
      (bind _asw_interact (Utilities|Casting|CastToW_Interact (UserInterface|GetUserWidgetObject (Variables|Default|GetWidget))))
      (Default|UpdateKey _asw_interact Key "to save"))
    (:NewEnumerator1
      (Rendering|SetVisibility _widget false false))))

(fn ConstructionScript)

(fn MSGGetDestroyedLoot
  (return 0))

(fn MSGGetEquippedWeapon
  (return ""))

(fn MSGGetInventory
  (return 0))

(fn MSGGetStats
  (return 0.0 0.0 0.0))