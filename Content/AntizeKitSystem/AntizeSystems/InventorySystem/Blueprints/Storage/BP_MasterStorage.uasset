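; Base storage container actor for the inventory system, with a configurable mesh and an "open" key prompt shown while the player is in interaction radius.
; On BeginPlay, a non-global storage sizes its BPStorage component, seeds it with DT_Item-validated default items capped at max stack, then loads its slots.
; DoSaveStorage passes saving to the component.
; Global storage skips seeding, loading and saving here, and construction clears its default items.
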(event EventMSGInteraction
  (params (Interaction :type E_Interaction%20Enum :default "NewEnumerator0") (Amount :type Integer) (FromActor :type Actor%20Object%20Reference) (Key :type Text))
  (bind _widget (Variables|Default|GetWidget))
  ;[1 1 1] Show/Hide Interact text
  (switch Utilities|FlowControl|Switch|SwitchonE_Interaction Interaction
    (:NewEnumerator0
      (Rendering|SetVisibility _widget true false)
      (bind _asw_interact (Utilities|Casting|CastToW_Interact (UserInterface|GetUserWidgetObject (Variables|Default|GetWidget))))
      (Default|UpdateKey _asw_interact Key "to open"))
    (:NewEnumerator1
      (Rendering|SetVisibility _widget false false))))

(event EventBeginPlay
  ;[1 1 1] Constructeur - If not global inventory, load storage slot
  ;;[1 1 1] Hide debug text
  (Rendering|SetVisibility (Variables|Default|GetTextRender) false false)
  (if (Utilities|Enum|NotEqual(Enum) (Variables|Setting|GetStorageName) "NewEnumerator0")
    (Variables|/Game/AntizeKitSystem/AntizeSystems/InventorySystem/Blueprints/Storage/BP_StorageComponent.BP_StorageComponent_C|SetStorageName (Variables|Default|GetBP_Storage) (Variables|Setting|GetStorageName))
    (CallFunction|CleanDefaultItem)
    (Default|LoadStorageSlots (Variables|Default|GetBP_Storage))))

(fn ConstructionScript
  (bind _staticmeshcorrection (Variables|Setting|MeshAndText|GetStaticMeshCorrection))
  (bind (_location _rotation _scale) (Utilities|Struct|BreakS_Correction _staticmeshcorrection))
  (Utilities|FlowControl|Sequence
    (:then_0
      ;[1 1 1] Set static mesh setting
      (Components|StaticMesh|SetStaticMesh (Variables|Default|GetCube) (Variables|Setting|MeshAndText|GetStaticMesh))
      (Transformation|SetRelativeTransform (Variables|Default|GetCube) (Math|Transform|MakeTransform _location _rotation _scale) false false)
      (Transformation|SetRelativeLocation (Variables|Default|GetWidget) (Variables|Setting|MeshAndText|GetPickUpTextLocCorrection) false false))
    (:then_1
      ;[1 1 1] Disable or restore default settings on GlobalStorage Name
      (if (Utilities|Enum|Equal(Enum) (Variables|Setting|GetStorageName) "NewEnumerator0")
        (Variables|Setting|SetStorageName "NewEnumerator0")
        (Utilities|Array|Clear (Variables|Setting|GetDefaultItem))
        (elif (Utilities|Enum|Equal(Enum) (Variables|Setting|GetStorageName) "NewEnumerator0")
          (Variables|Setting|SetStorageName "NewEnumerator1"))))))

(fn DoSaveStorage
  (params (SaveRef :type BP%20Save%20Inventory%20Object%20Reference))
  ;[1 1 1] If not GlobalStorage call SaveSlots
  (if (Utilities|Enum|NotEqual(Enum) (Variables|Setting|GetStorageName) "NewEnumerator0")
    (Default|DoSaveStorageSlots (Variables|Default|GetBP_Storage) SaveRef)
    (return)
    (else
      (return))))

(fn CleanDefaultItem
  (bind _local_defaultitem (LocalVariables|GetLocal_DefaultItem))
  (bind _bp_storage (Variables|Default|GetBP_Storage))
  (bind _bp_storage_2 (Variables|Default|GetBP_Storage))
  (bind _storageslots (Variables|/Game/AntizeKitSystem/AntizeSystems/InventorySystem/Blueprints/Storage/BP_StorageComponent.BP_StorageComponent_C|GetStorageSlots _bp_storage))
  (bind _returnvalue (Utilities|Array|Length _storageslots))
  ;[1 1 1] Resize storage size
  (bind _output_get (Variables|/Game/AntizeKitSystem/AntizeSystems/InventorySystem/Blueprints/Storage/BP_StorageComponent.BP_StorageComponent_C|SetStorageSize _bp_storage_2 (Variables|Setting|GetStorageSize)))
  (Utilities|Array|Resize (Variables|/Game/AntizeKitSystem/AntizeSystems/InventorySystem/Blueprints/Storage/BP_StorageComponent.BP_StorageComponent_C|GetStorageSlots _bp_storage_2) _output_get)
  ;[1 1 1] Continue if array have default item
  (if (> (Utilities|Array|Length (Variables|Setting|GetDefaultItem)) 0)
    ;[1 1 1] Check for valid and amount item
    (for _array_element (Variables|Setting|GetDefaultItem)
      (LocalVariables|SetLocal_Slot _array_element)
      (bind _returnvalue_2 (Utilities|GetDataTableRow "/Game/AntizeKitSystem/AntizeSystems/InventorySystem/Logics/Datatable/DT_Item.DT_Item" (.RowName (Utilities|Struct|BreakDataTableRowHandle (.Item (Utilities|Struct|BreakS_InventorySlot _array_element)))))
        (:then
          (if (> (.Amount (Utilities|Struct|BreakS_InventorySlot _array_element)) 0)
            (if (> (Utilities|Struct|BreakS_InventorySlot (LocalVariables|GetLocal_Slot)) (Utilities|Struct|BreakS_Item _returnvalue_2))
              (Utilities|Array|Add _local_defaultitem (Utilities|Struct|MakeS_InventorySlot (.Item (Utilities|Struct|BreakS_InventorySlot (LocalVariables|GetLocal_Slot))) (Utilities|Struct|BreakS_Item _returnvalue_2) (.Ammo (Utilities|Struct|BreakS_InventorySlot (LocalVariables|GetLocal_Slot)))))
              (else
                (Utilities|Array|Add _local_defaultitem (LocalVariables|GetLocal_Slot))))))))
    ;[1 1 1] Continue if array have item
    (if (> (Utilities|Array|Length (LocalVariables|GetLocal_DefaultItem)) 0)
      ;[1 1 1] Resize if defaut item lenght are over storage lenght
      (if (> (Utilities|Array|Length (LocalVariables|GetLocal_DefaultItem)) _returnvalue)
        (Utilities|Array|Resize (LocalVariables|GetLocal_DefaultItem) _returnvalue))
      ;[1 1 1] Add item
      (for (_array_element_2 _array_index) (LocalVariables|GetLocal_DefaultItem)
        (Utilities|Array|SetArrayElem (Variables|/Game/AntizeKitSystem/AntizeSystems/InventorySystem/Blueprints/Storage/BP_StorageComponent.BP_StorageComponent_C|GetStorageSlots (Variables|Default|GetBP_Storage)) _array_index _array_element_2))
      (return)
      (else
        (return)))
    (else
      (return))))

(fn MSGGetDestroyedLoot
  (return 0))

(fn MSGGetEquippedWeapon
  (return ""))

(fn MSGGetInventory
  (return 0))

(fn MSGGetStats
  (return 0.0 0.0 0.0))