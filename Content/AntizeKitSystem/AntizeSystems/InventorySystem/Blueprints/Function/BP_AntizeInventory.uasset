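; Function library for the Antize inventory system, with helpers for slot widgets, item data and save games.
; LoadSlots loads or creates a BP_SaveInventory by slot name, and SaveSlots updates its count, date and saved flag before writing it.
; Other helpers reset inventory or storage slot styles, read item names from DT_Item and map values to red-to-green colors.
; Duplicate-save logic in SaveSlots is disconnected.
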(fn ResetSyleonSlot
  (params (Object :type Widget%20Object%20Reference))
  (bind _asw_inventory_slot (Utilities|Casting|CastToW_InventorySlot Object)
    (:then
      (Default|ResetInventorySlotStyle _asw_inventory_slot))
    (:CastFailed
      (bind _asw_storage_slot (Utilities|Casting|CastToW_StorageSlot Object)
        (:then
          (Default|ResetStorageSlotStyle _asw_storage_slot))
        (:CastFailed
          (return)))))
  (return))

(fn LoadSlots
  (params (SlotName :type String))
  ;[1 1 1] Get slot
  (LocalVariables|SetLocal_SlotName SlotName)
  ;[1 1 1] Check if save exist
  (bind _returnvalue (SaveGame|DoesSaveGameExist (LocalVariables|GetLocal_SlotName)))
  (if _returnvalue
    ;[1 1 1] Load save
    (bind _returnvalue_2 (SaveGame|LoadGamefromSlot (LocalVariables|GetLocal_SlotName)))
    (bind _asbp_save_inventory (Utilities|Casting|CastToBP_SaveInventory _returnvalue_2)
      (:then
        (return _asbp_save_inventory))
      (:CastFailed
        (return 0)))
    (else
      ;[1 1 1] Create new save
      (bind _returnvalue_3 (SaveGame|CreateSaveGameObject "/Game/AntizeKitSystem/AntizeSystems/InventorySystem/Blueprints/SaveGame/BP_SaveInventory.BP_SaveInventory_C"))
      (return _returnvalue_3))))

(fn SaveSlots
  (params (IsNewGame? :type Boolean) (Save :type BP%20Save%20Inventory%20Object%20Reference))
  (LocalVariables|SetLocal_Save Save)
  (if IsNewGame?
    _
    (else
      (Variables|/Game/AntizeKitSystem/AntizeSystems/InventorySystem/Blueprints/SaveGame/BP_SaveInventory.BP_SaveInventory_C|SetSaved? (LocalVariables|GetLocal_Save) true)))
  (Math|Integer|IncrementInt (Variables|/Game/AntizeKitSystem/AntizeSystems/InventorySystem/Blueprints/SaveGame/BP_SaveInventory.BP_SaveInventory_C|GetNumberSave (LocalVariables|GetLocal_Save))
    (:%20%20
      (Variables|/Game/AntizeKitSystem/AntizeSystems/InventorySystem/Blueprints/SaveGame/BP_SaveInventory.BP_SaveInventory_C|SetDateSaved (LocalVariables|GetLocal_Save) (Math|DateTime|Now))
      (bind _returnvalue (SaveGame|SaveGametoSlot (LocalVariables|GetLocal_Save) (Variables|/Game/AntizeKitSystem/AntizeSystems/InventorySystem/Blueprints/SaveGame/BP_SaveInventory.BP_SaveInventory_C|GetSlotName (LocalVariables|GetLocal_Save))))
      (return _returnvalue))))

(fn GetNamefromDatatable
  (params (ItemDB :type Data%20Table%20Row%20Handle%20Structure))
  (bind _returnvalue (Utilities|GetDataTableRow "/Game/AntizeKitSystem/AntizeSystems/InventorySystem/Logics/Datatable/DT_Item.DT_Item" (Utilities|Struct|BreakDataTableRowHandle ItemDB))
    (:then
      (return (Utilities|Struct|BreakS_Item _returnvalue)))
    (:RowNotFound
      (return "Not found"))))

(fn GetColorbyValue
  (params (Value :type Float%20%28single-precision%29))
  (return (select (<= Value 0.1) "(R=1.000000,G=0.000000,B=0.000000,A=1.000000)" (select (<= Value 0.3) "(R=1.000000,G=0.058824,B=0.000000,A=1.000000)" (select (<= Value 0.5) "(R=1.000000,G=0.345098,B=0.000000,A=1.000000)" (select (<= Value 0.6) "(R=0.992157,G=1.000000,B=0.003922,A=1.000000)" (select (<= Value 0.95) "(R=0.674510,G=1.000000,B=0.000000,A=1.000000)" "(R=0.050980,G=1.000000,B=0.000000,A=1.000000)")))))))