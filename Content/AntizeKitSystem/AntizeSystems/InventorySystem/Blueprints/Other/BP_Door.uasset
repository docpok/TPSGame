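; BP_Door is an interactable swinging door with a configurable mesh, shown with a key prompt widget while in interaction radius.
; Server_DoorOpenClose runs on authority, refusing while locked or animating.
; A timeline lerps the Porteur component's yaw between zero and MaxRotate, and a fixed delay then flips the Open state.
; The open or close sound is sent through the interacting actor via an interface message.
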(event Custom|ResetVarAfterOpenClose
  ;[1 1 1] Reset variables after open/close
  (Networking|SwitchHasAuthority
    (:Authority
      (Variables|Traitement|SetOpen? (not (Variables|Traitement|GetOpen?)))
      (Variables|Traitement|SetInAnim? false))))

(event Custom|Server_DoorOpenClose
  (params (FromActorRef :type Actor%20Object%20Reference))
  ;[1 1 1] Open/Close door (Replicated)
  (Networking|SwitchHasAuthority
    (:Authority
      (bind _canopen_ (CallFunction|GetCanOpenClose))
      (if _canopen_
        (Variables|Traitement|SetInAnim? true)
        (Utilities|FlowControl|Sequence
          (:then_0
            (CallFunction|OpenCloseAnim)
            (Utilities|FlowControl|Delay 0.75)
            (CallFunction|ResetVarAfterOpenClose))
          (:then_1
            (Utilities|IsValid FromActorRef
              (:Is%20Valid
                (Class|BPAntizeInventoryInterface|MSGPlaySoundatLocation(Message) FromActorRef (select (Variables|Traitement|GetOpen?) "/Game/AntizeKitSystem/AntizeSystems/InventorySystem/Ressources/Audio/Cue_DoorClose.Cue_DoorClose" "/Game/AntizeKitSystem/AntizeSystems/InventorySystem/Ressources/Audio/Cue_DoorOpen.Cue_DoorOpen") (Transformation|GetActorLocation))))))))))

(event Custom|OpenCloseAnim
  (bind _maxrotate (Variables|Setting|GetMaxRotate))
  (bind _returnvalue (Math|Rotator|MakeRotator 0.0 0.0 _maxrotate))
  ;[1 1 1] Open/Close anim
  (Networking|SwitchHasAuthority
    (:Authority
      (bind _alpha (Timeline|Timeline_0 PlayFromStart)
        (:Update
          (Transformation|SetRelativeRotation (Variables|Default|GetPorteur) (select (Variables|Traitement|GetOpen?) (Math|Rotator|Lerp(Rotator) _returnvalue "0, 0, 0" _alpha) (Math|Rotator|Lerp(Rotator) "0, 0, 0" _returnvalue _alpha)) false false))))))

(event EventMSGInteraction
  (params (Interaction :type E_Interaction%20Enum :default "NewEnumerator0") (Amount :type Integer) (FromActor :type Actor%20Object%20Reference) (Key :type Text))
  (bind _widget (Variables|Default|GetWidget))
  ;[1 1 1] Show/Hide Interact text
  (switch Utilities|FlowControl|Switch|SwitchonE_Interaction Interaction
    (:NewEnumerator0
      (Rendering|SetVisibility _widget true false)
      (bind _asw_interact (Utilities|Casting|CastToW_Interact (UserInterface|GetUserWidgetObject (Variables|Default|GetWidget))))
      (Default|UpdateKey _asw_interact Key "to interact"))
    (:NewEnumerator1
      (Rendering|SetVisibility _widget false false))))

(fn ConstructionScript
  (Components|StaticMesh|SetStaticMesh (Variables|Default|GetStaticMesh) (Variables|Setting|GetMesh)))

(fn GetCanOpenClose
  (if (Variables|Traitement|GetInAnim?)
    (return false)
    (elif (Variables|Setting|GetLocked?)
      (return false)
      (else
        (return true)))))

(fn MSGGetDestroyedLoot
  (return 0))

(fn MSGGetEquippedWeapon
  (return ""))

(fn MSGGetInventory
  (return 0))

(fn MSGGetStats
  (return 0.0 0.0 0.0))