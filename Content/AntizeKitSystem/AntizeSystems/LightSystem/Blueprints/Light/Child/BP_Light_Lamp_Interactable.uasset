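; Interactable lamp Blueprint in the light system that carries its own light switch as a child actor.
; The construction script adds the lamp to the switch's LightLinked array and, on authority only, copies the lamp's Enabled value to the switch.
; MSGOpacity events are forwarded to the switch child actor, and BeginPlay only calls the parent.
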(event EventBeginPlay
  (|CallParentFunction))

(event Collision|EventActorBeginOverlap
  (params (OtherActor :type Actor%20Object%20Reference)))

(event EventTick
  (params (DeltaSeconds :type Float%20%28single-precision%29)))

(event EventMSGOpacity
  (params (Show? :type Boolean) (PlayerRef :type Actor%20Object%20Reference) (Opacity :type Float%20%28single-precision%29))
  (Class|BPAntizeLightInterface|MSGOpacity(Message) (Variables|/Script/Engine.ChildActorComponent|GetChildActor (Variables|Default|GetMaster_LightSwitch)) Show? PlayerRef Opacity))

(fn ConstructionScript
  (|CallParentFunction)
  (bind _asmaster_light_switch (Utilities|Casting|CastToMaster_LightSwitch (Variables|/Script/Engine.ChildActorComponent|GetChildActor (Variables|Default|GetMaster_LightSwitch))))
  (Utilities|Array|AddUnique (Variables|/Game/AntizeKitSystem/AntizeSystems/LightSystem/Blueprints/LightSwitch/Master_LightSwitch.Master_LightSwitch_C|GetLight%20Linked _asmaster_light_switch) self)
  (Networking|SwitchHasAuthority
    (:Authority
      (bind _asmaster_light_switch_2 (Utilities|Casting|CastToMaster_LightSwitch (Variables|/Script/Engine.ChildActorComponent|GetChildActor (Variables|Default|GetMaster_LightSwitch))))
      (Variables|/Game/AntizeKitSystem/AntizeSystems/LightSystem/Blueprints/LightSwitch/Master_LightSwitch.Master_LightSwitch_C|SetEnabled? _asmaster_light_switch_2 (Variables|Default|GetEnabled?)))))