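; Master light switch actor that works as either an interactable wall switcher or a pawn-triggered collision box with normal, timed, on-only and off-only modes.
; The server owns the state and messages linked lights, optional inverse lights and linked switches.
; Switchers multicast indicator color and prompt text, with the prompt widget fading by distance after a visibility trace.
; The construction script configures components for the chosen type and deduplicates link arrays.
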(event OnComponentEndOverlap(CollisionBox)
  (params (OverlappedComponent :type Primitive%20Component%20Object%20Reference) (OtherActor :type Actor%20Object%20Reference) (OtherComp :type Primitive%20Component%20Object%20Reference) (OtherBodyIndex :type Integer))
  ;[0.15 1 0.5] Server (Only) -> Bengin/End overlap (Called by player collision)
  (Networking|SwitchHasAuthority
    (:Authority
      (if (Utilities|Enum|Equal(Enum) (Variables|Setting|GetLight%20Switch%20Type) "NewEnumerator1")
        (Utilities|IsValid OtherActor
          (:Is%20Valid
            (Utilities|Casting|CastToPawn OtherActor)
            (switch Utilities|FlowControl|Switch|SwitchonE_SwticherCollisionType (Variables|Setting|ColliionBox|GetCollision%20Box%20Type)
              (:NewEnumerator5
                (if (Variables|Setting|GetEnabled?)
                  (Variables|Setting|SetEnabled? false)
                  (CallFunction|EnableDisableLinkedLight true))))))))))

(event OnComponentBeginOverlap(CollisionBox)
  (params (OverlappedComponent :type Primitive%20Component%20Object%20Reference) (OtherActor :type Actor%20Object%20Reference) (OtherComp :type Primitive%20Component%20Object%20Reference) (OtherBodyIndex :type Integer) (bFromSweep :type Boolean) (SweepResult :type Hit%20Result%20Structure%20%28by%20ref%29))
  ;[0.15 1 0.5] Server (Only) -> Bengin/End overlap (Called by player collision)
  (Networking|SwitchHasAuthority
    (:Authority
      (if (Utilities|Enum|Equal(Enum) (Variables|Setting|GetLight%20Switch%20Type) "NewEnumerator1")
        (Utilities|IsValid OtherActor
          (:Is%20Valid
            (Utilities|Casting|CastToPawn OtherActor)
            (switch Utilities|FlowControl|Switch|SwitchonE_SwticherCollisionType (Variables|Setting|ColliionBox|GetCollision%20Box%20Type)
              (:NewEnumerator5
                (if (not (Variables|Setting|GetEnabled?)) :!label _label
                  (Variables|Setting|SetEnabled? true :!label _label_2)
                  (CallFunction|EnableDisableLinkedLight true :!label _label_3)))
              (:NewEnumerator0
                (Utilities|FlowControl|Sequence
                  (:then_0
                    (Utilities|FlowControl|RetriggerableDelay 0.1)
                    (Variables|Traitement|OnDelay|SetCanceled? false)
                    (Utilities|FlowControl|RetriggerableDelay (Variables|Setting|ColliionBox|GetKeep%20Duration))
                    (if (not (Variables|Traitement|OnDelay|GetCanceled?))
                      (Variables|Setting|SetEnabled? false)
                      (CallFunction|DoCollisionInteract)))
                  (:then_1
                    (goto _label_2))))
              (:NewEnumerator4
                (if (Variables|Setting|GetEnabled?)
                  (Variables|Setting|SetEnabled? false)
                  (goto _label_3)))
              (:NewEnumerator1
                (goto _label)))))))))

(event Custom|Client_UpdateWidget
  (params (Enabled? :type Boolean))
  ;[0.2 0.9 1] Multi -> Client -> Update the widget
  (Class|BPAntizeLightInterface|MSGUpdate(Message) (UserInterface|GetUserWidgetObject (Variables|Default|GetWidget)) (Variables|Traitement|byPlayer|GetInLineTrace?) (CallFunction|GetWidgetText Enabled?)))

(event Custom|Multi_RefreshIndicatorLight
  (params (Enabled? :type Boolean))
  ;[0.1294 1 0.0152] Multi -> Refresh everyone's indicator light
  (Rendering|Material|SetVectorParameterValue (Variables|Traitement|GetIndicatorLightMaterial) "Color" (select Enabled? "(R=0.000000,G=1.000000,B=0.000000,A=1.000000)" "(R=1.000000,G=0.000000,B=0.000000,A=1.000000)") :!class /Script/Engine.MaterialInstanceDynamic))

(event Custom|Server_RefreshIndicatorLight
  ;[0.1294 1 0.0152] Multi -> Refresh everyone's indicator light
  (Networking|SwitchHasAuthority
    (:Authority
      (if (Utilities|Enum|Equal(Enum) (Variables|Setting|GetLight%20Switch%20Type) "NewEnumerator0")
        (CallFunction|MultiRefreshIndicatorLight (Variables|Setting|GetEnabled?))))))

(event Custom|Server_UpdateWidget
  ;[0.2 0.9 1] Multi -> Client -> Update the widget
  (Networking|SwitchHasAuthority
    (:Authority
      (if (and (Variables|Setting|Widget|GetShow%20Widget?) (Utilities|Enum|Equal(Enum) (Variables|Setting|GetLight%20Switch%20Type) "NewEnumerator0"))
        (CallFunction|MultiUpdateWidget (Variables|Setting|GetEnabled?))))))

(event Custom|DoCollisionInteract
  ;[0.15 1 0.5] Server (Only) -> Bengin/End overlap (Called by player collision)
  (Networking|SwitchHasAuthority
    (:Authority
      (CallFunction|EnableDisableLinkedLight true))))

(event Custom|Multi_UpdateWidget
  (params (Enabled? :type Boolean))
  ;[0.2 0.9 1] Multi -> Client -> Update the widget
  (CallFunction|ClientUpdateWidget Enabled?))

(event EventMSGUpdate
  (params (ShowAction? :type Boolean) (ActionText :type Text))
  ;[0.15 1 0.5] Server -> Update (Called by LightSwitch)
  (Networking|SwitchHasAuthority
    (:Authority
      (Variables|Setting|SetEnabled? ShowAction?)
      (CallFunction|ServerRefreshIndicatorLight)
      (Variables|Traitement|OnDelay|SetCanceled? true))))

(event EventMSGOpacity
  (params (Show? :type Boolean) (PlayerRef :type Actor%20Object%20Reference) (Opacity :type Float%20%28single-precision%29))
  ;[0.2 0.9 1] Client -> Set Widget opacity (Called by player)
  (if (Variables|Setting|Widget|GetShow%20Widget?)
    (CallFunction|RefreshWidgetOpacity Show? PlayerRef Opacity)))

(event EventMSGonLineTraceChanged
  (params (InLinetrace? :type Boolean) (Message :type Text))
  ;[0.2 0.9 1] Client -> Actor are in Player linetrace (Called by player)
  (Variables|Traitement|ByPlayer|SetActionKey Message)
  (if InLinetrace?
    (if (not (Variables|Traitement|byPlayer|GetInLineTrace?))
      (Variables|Traitement|byPlayer|SetInLineTrace? true)
      (if (Variables|Setting|Widget|GetShow%20Widget?) :!label _label
        (Class|BPAntizeLightInterface|MSGUpdate(Message) (UserInterface|GetUserWidgetObject (Variables|Default|GetWidget)) (Variables|Traitement|byPlayer|GetInLineTrace?) (CallFunction|GetWidgetText (Variables|Setting|GetEnabled?)))))
    (elif (Variables|Traitement|byPlayer|GetInLineTrace?)
      (Variables|Traitement|byPlayer|SetInLineTrace? false)
      (goto _label))))

(event EventBeginPlay
  ;[0.1294 1 0.0152] Constructeur - Update all light and update widget if switcher
  (Utilities|FlowControl|Sequence
    (:then_0
      (CallFunction|EnableDisableLinkedLight false))
    (:then_1
      (if (and (Variables|Setting|Widget|GetShow%20Widget?) (Utilities|Enum|Equal(Enum) (Variables|Setting|GetLight%20Switch%20Type) "NewEnumerator0"))
        (bind _asw_interactive_name (Utilities|Casting|CastToW_InteractiveName (UserInterface|GetUserWidgetObject (Variables|Default|GetWidget))))
        (Default|StartUp _asw_interactive_name (Variables|Setting|Widget|GetLight%20Switch%20Name))))))

(event EventMSGInteract
  (params (Variable :type Boolean) (PlayerRef :type Character%20Object%20Reference))
  ;[0.15 1 0.5] Server -> Interact (Called by player and collision)
  (Networking|SwitchHasAuthority
    (:Authority
      (Utilities|FlowControl|Sequence
        (:then_0
          (Variables|Setting|SetEnabled? (not (Variables|Setting|GetEnabled?)))
          (CallFunction|ChangeLightSwitch)
          (CallFunction|ServerRefreshIndicatorLight)
          (Utilities|FlowControl|Sequence
            (:then_0
              (CallFunction|EnableDisableLinkedLight true))
            (:then_1
              (CallFunction|ServerUpdateWidget))))
        (:then_1
          (if (Utilities|Enum|Equal(Enum) (Variables|Setting|GetLight%20Switch%20Type) "NewEnumerator0")
            (Utilities|IsValid PlayerRef
              (:Is%20Valid
                (Class|BPAntizeInventoryInterface|MSGPlaySoundatLocation(Message) PlayerRef "/Game/AntizeKitSystem/AntizeSystems/LightSystem/Resource/Sounds/Cue_Turn_Light.Cue_Turn_Light" (Transformation|GetActorLocation))))))))))

(fn ConstructionScript
  (bind _sm_lightswitch_movable (Variables|Setting|Mesh|GetSM%20LightSwitch%20Movable))
  (bind _sm_lightswitch (Variables|Setting|Mesh|GetSM%20LightSwitch))
  (bind _collisionbox (Variables|Default|GetCollisionBox))
  (Utilities|FlowControl|Sequence
    (:then_0
      ;[1 1 1] Refresh light switch and create indicator material (Everybody)
      (if (Utilities|Enum|Equal(Enum) (Variables|Setting|GetLight%20Switch%20Type) "NewEnumerator0")
        (bind _returnvalue (Rendering|Material|CreateDynamicMaterialInstance (Variables|Default|GetIndicatorLight) 0 "/Game/AntizeKitSystem/AntizeSystems/LightSystem/Resource/Materials/M_MasterEmissive.M_MasterEmissive" "None" :!class /Script/Engine.PrimitiveComponent))
        (bind _output_get (Variables|Traitement|SetIndicatorLightMaterial _returnvalue))
        (Rendering|Material|SetScalarParameterValue _output_get "EmissivePower" 5e+01 :!class /Script/Engine.MaterialInstanceDynamic)
        (Rendering|Material|SetVectorParameterValue (Variables|Traitement|GetIndicatorLightMaterial) "Color" (select (Variables|Setting|GetEnabled?) "(R=0.000000,G=1.000000,B=0.000000,A=1.000000)" "(R=1.000000,G=0.000000,B=0.000000,A=1.000000)") :!class /Script/Engine.MaterialInstanceDynamic)
        (Rendering|Material|SetScalarParameterValue (Variables|Traitement|GetIndicatorLightMaterial) "UseFlickering?" 1.0 :!class /Script/Engine.MaterialInstanceDynamic)
        (Utilities|FlowControl|Sequence
          (:then_0
            ;[1 1 1] Disable widget if not enabled
            (if (not (Variables|Setting|Widget|GetShow%20Widget?))
              (Rendering|SetVisibility (Variables|Default|GetWidget) false false)))
          (:then_1
            ;[1 1 1] Disable indicator if not enabled
            (if (not (Variables|Setting|Mesh|GetShow%20Indicator?))
              (Rendering|SetVisibility (Variables|Default|GetIndicatorLight) false false)
              (Collision|SetCollisionEnabled (Variables|Default|GetIndicatorLight) "NoCollision")
              (else
                (Transformation|SetRelativeTransform (Variables|Default|GetIndicatorLight) (Variables|Setting|Mesh|GetIndicator%20Correction) false false)
                (CallFunction|ChangeLightSwitch)))))))
    (:then_1
      ;[1 1 1] Disable component
      (if (Utilities|Enum|Equal(Enum) (Variables|Setting|GetLight%20Switch%20Type) "NewEnumerator1")
        (Rendering|SetVisibility (Variables|Default|GetLightSwitch) false false)
        (Collision|SetCollisionEnabled (Variables|Default|GetIndicatorLight) "NoCollision")
        (else
          (Rendering|SetVisibility _collisionbox false false)
          (Collision|SetCollisionEnabled _collisionbox "NoCollision"))))
    (:then_2
      ;[1 1 1] Setting up Static Mesh or Collision Box
      (if (Utilities|Enum|Equal(Enum) (Variables|Setting|GetLight%20Switch%20Type) "NewEnumerator0")
        (Transformation|SetRelativeTransform (Utilities|Select :Index (Variables|Setting|GetLight%20Switch%20Type) :NewEnumerator0 (Variables|Default|GetLightSwitch) :NewEnumerator1 (Variables|Default|GetCollisionBox)) (Variables|Setting|Mesh|GetSM%20Correction) false false)
        (Transformation|SetRelativeTransform (Variables|Default|GetCollision) (Variables|Setting|Mesh|GetCollision%20Correction) false false)
        (Utilities|FlowControl|Sequence
          (:then_0
            (Components|StaticMesh|SetStaticMesh (Variables|Default|GetLightSwitchMovable) (select (Utilities|IsValid _sm_lightswitch_movable) _sm_lightswitch_movable "/Game/AntizeKitSystem/AntizeSystems/LightSystem/Resource/StaticMesh/SM_Empty.SM_Empty")))
          (:then_1
            (Components|StaticMesh|SetStaticMesh (Variables|Default|GetLightSwitch) (select (Utilities|IsValid _sm_lightswitch) _sm_lightswitch "/Game/AntizeKitSystem/AntizeSystems/LightSystem/Resource/StaticMesh/SM_Empty.SM_Empty"))))
        (else
          (Transformation|SetRelativeTransform (Variables|Default|GetCollisionBox) (Variables|Setting|ColliionBox|GetCollision%20Box%20Correction) false false)
          (Components|StaticMesh|SetStaticMesh (Variables|Default|GetLightSwitch) "/Game/AntizeKitSystem/AntizeSystems/LightSystem/Resource/StaticMesh/SM_Empty.SM_Empty")
          (Components|StaticMesh|SetStaticMesh (Variables|Default|GetLightSwitchMovable) "/Game/AntizeKitSystem/AntizeSystems/LightSystem/Resource/StaticMesh/SM_Empty.SM_Empty"))))
    (:then_3
      ;[1 1 1] Clean linked array
      (for _array_element (Variables|Setting|GetLight%20Switch%20Linked)
        (if (!= _array_element self)
          (Utilities|Array|AddUnique (LocalVariables|GetLocal_Switcher) _array_element)))
      (Variables|Setting|SetLight%20Switch%20Linked (LocalVariables|GetLocal_Switcher))
      (for _array_element_2 (Variables|Setting|GetLight%20Linked)
        (Utilities|Array|AddUnique (LocalVariables|GetLocal_Light) _array_element_2))
      (Variables|Setting|SetLight%20Linked (LocalVariables|GetLocal_Light))
      (for _array_element_3 (Variables|Setting|GetInversed%20Light%20Linked)
        (Utilities|Array|AddUnique (LocalVariables|GetLocal_InversedLight) _array_element_3))
      (Variables|Setting|SetInversed%20Light%20Linked (LocalVariables|GetLocal_InversedLight))
      ;[1 1 1] Refresh all switcher linked
      (if (Variables|Setting|GetRefresh)
        (Variables|Setting|SetRefresh false)
        (for _array_element_4 (Variables|Setting|GetLight%20Switch%20Linked)
          (Class|BPAntizeLightInterface|MSGUpdate(Message) _array_element_4 (Variables|Setting|GetEnabled?)))))))

(fn ChangeLightSwitch
  ;[1 1 1] Update mesh if switcher
  (if (Utilities|Enum|Equal(Enum) (Variables|Setting|GetLight%20Switch%20Type) "NewEnumerator0")
    (bind _output_get (Variables|Traitement|SetMyFlipFlop (not (Variables|Traitement|GetMyFlipFlop))))
    (Transformation|SetRelativeRotation (Variables|Default|GetLightSwitchMovable) (Math|Rotator|MakeRotator 0.0 (select _output_get 1.8e+02 0.0) 0.0) false false)
    (return)
    (else
      (return))))

(fn GetWidgetText
  (params (Enabled? :type Boolean))
  (return (Utilities|Text|FormatText "\"{Action}\" {Message}" (Variables|Traitement|ByPlayer|GetActionKey) (select Enabled? "turn off" "turn on"))))

(fn RefreshWidgetOpacity
  (params (Show? :type Boolean) (PlayerRef :type Actor%20Object%20Reference) (Opacity :type Float%20%28single-precision%29))
  (bind _lightswitch (Variables|Default|GetLightSwitch))
  (bind _widget (Variables|Default|GetWidget))
  (bind _returnvalue (Transformation|GetWorldLocation _lightswitch))
  ;[1 1 1] Check if actor is in sight and set opacity
  (if Show?
    (bind _output_get (LocalVariables|SetLocal_PlayerRef PlayerRef))
    (LocalVariables|SetLocal_PlayerLocation (Transformation|GetActorLocation _output_get))
    (bind (_outhit _returnvalue_2) (Collision|LineTraceByChannel (LocalVariables|GetLocal_PlayerLocation) _returnvalue "TraceTypeQuery1" false (Utilities|Array|MakeArray (LocalVariables|GetLocal_PlayerRef)) "None" false "(R=0.000000,G=0.637930,B=1.000000,A=1.000000)" "(R=1.000000,G=0.000000,B=0.750000,A=1.000000)" 1e+01))
    (if _returnvalue_2
      (Rendering|SetVisibility _widget (== (.HitActor (Collision|BreakHitResult _outhit)) self) false)
      (if (== (.HitActor (Collision|BreakHitResult _outhit)) self)
        (Class|BPAntizeLightInterface|MSGOpacity(Message) (UserInterface|GetUserWidgetObject _widget) false 0 (Math|Float|Clamp(Float) (- 1.0 (/ (- (Math|Vector|VectorLength (- _returnvalue (LocalVariables|GetLocal_PlayerLocation))) (Variables|Setting|Widget|GetFade%20Start%20Distance)) (Variables|Setting|Widget|GetFade%20Distance))))))
      (else
        (Rendering|SetVisibility (Variables|Default|GetWidget) false false)))
    (else
      (Rendering|SetVisibility (Variables|Default|GetWidget) false false))))

(fn EnableDisableLinkedLight
  (params (RefreshSwitcher? :type Boolean))
  ;[1 1 1] Only on server
  (Networking|SwitchHasAuthority
    (:Authority
      (Utilities|FlowControl|Sequence
        (:then_0
          (for _array_element (Variables|Setting|GetLight%20Linked)
            (Utilities|IsValid _array_element
              (:Is%20Valid
                (Class|BPAntizeLightInterface|MSGInteract(Message) _array_element (Variables|Setting|GetEnabled?)))))
          (if (Variables|Setting|GetInversed?)
            (for _array_element_2 (Variables|Setting|GetInversed%20Light%20Linked)
              (Utilities|IsValid _array_element_2
                (:Is%20Valid
                  (Class|BPAntizeLightInterface|MSGInteract(Message) _array_element_2 (not (Variables|Setting|GetEnabled?))))))))
        (:then_1
          (if RefreshSwitcher?
            (for _array_element_3 (Variables|Setting|GetLight%20Switch%20Linked)
              (Utilities|IsValid _array_element_3
                (:Is%20Valid
                  (Class|BPAntizeLightInterface|MSGUpdate(Message) _array_element_3 (Variables|Setting|GetEnabled?)))))))))))