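; Blueprint interface for the Antize Kit chat system, declaring the messaging contract used between chat participants.
; It covers delivering new messages with category, sender, recipient, name and prefix, requesting private messages, and listing connected players.
; It also exposes getters and setters for player ID and team with color ID, username lookups, and an emote trigger.
; All functions are empty declarations or default returns, leaving behavior to implementers.
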(fn MSGNewMessage
  (params (Received? :type Boolean) (MessageCategory :type E_ChatCategory%20Enum :default "NewEnumerator3") (PlayerID :type Integer) (ToPlayerID :type Integer) (Username :type Text) (Message :type Text) (Prefix :type E_Prefix%20Enum :default "NewEnumerator0")))

(fn MSGGetConnectedPlayers
  (return 0))

(fn MSGSetPlayerID
  (params (PlayerID :type Integer)))

(fn MSGGetPlayerID
  (return 0))

(fn MSGRequestPrivateMessage
  (params (Request :type E_PrivateMessage%20Enum :default "NewEnumerator1") (ToPlayerID :type Integer) (Username :type Text) (Message :type Text))
  (return false))

(fn MSGGetPlayerIDfromUsername
  (params (Username :type Text))
  (return 0))

(fn MSGGetUsername
  (return false ""))

(fn MSGGetTeamID
  (return 0 0))

(fn MSGSetTeamID
  (params (TeamID :type Integer) (ColorID :type Integer))
  (return))

(fn MSGPlayEmote
  (params (EmoteToPlay :type E_Emote%20Enum :default "NewEnumerator0")))