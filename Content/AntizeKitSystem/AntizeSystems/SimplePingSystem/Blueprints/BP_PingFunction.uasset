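; Helper functions for the Simple Ping System that pick ping colors and test a ping's screen visibility.
; GetColorByID maps an ID to one of five preset colors.
; GetPingIsOnScreen projects the ping's location against viewport bounds, allowing fade only when right mouse is flagged and the ping sits in the central screen region.
; With DoAction set, on-screen pings also receive CalculeDistance and OnFade calls.
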(fn GetColorbyID
  (params (ColorID :type Integer))
  (return (Utilities|Select :Index ColorID :Option%200 "(R=1.000000,G=0.250000,B=0.000000,A=1.000000)" :Option%201 "(R=0.000000,G=0.250000,B=1.000000,A=1.000000)" :Option%202 "(R=1.000000,G=0.000000,B=0.250000,A=1.000000)" :Option%203 "(R=0.250000,G=1.000000,B=0.000000,A=1.000000)" :Option%204 "(R=0.588320,G=1.000000,B=0.250000,A=1.000000)")))

(fn GetPingIsonScreen
  (params (IsMouseR? :type Boolean) (PingRef :type BP%20Ping%20Object%20Reference) (DoAction? :type Boolean) (PlayerRef :type Player%20Controller%20Object%20Reference))
  (bind _returnvalue (Viewport|GetViewportSize PlayerRef))
  (bind _returnvalue_2 (Viewport|GetViewportSize PlayerRef))
  (LocalVariables|SetLocal_IsMouseR? IsMouseR?)
  (LocalVariables|SetLocal_PingRef PingRef)
  (LocalVariables|SetLocal_DoAction? DoAction?)
  (LocalVariables|SetLocal_ScreenLocation (.ScreenLocation (Class|PlayerController|ProjectWorldLocationtoScreen PlayerRef (Transformation|GetActorLocation (LocalVariables|GetLocal_PingRef)) false)))
  (if (Math|Boolean|ANDBoolean (> (.X (Math|Vector2D|BreakVector2D (LocalVariables|GetLocal_ScreenLocation))) 0.0) (< (.X (Math|Vector2D|BreakVector2D (LocalVariables|GetLocal_ScreenLocation))) (.x _returnvalue)) (> (.Y (Math|Vector2D|BreakVector2D (LocalVariables|GetLocal_ScreenLocation))) 0.0) (< (.Y (Math|Vector2D|BreakVector2D (LocalVariables|GetLocal_ScreenLocation))) (.y _returnvalue)))
    (if (LocalVariables|GetLocal_IsMouseR?)
      (if (Math|Boolean|ANDBoolean (> (.X (Math|Vector2D|BreakVector2D (LocalVariables|GetLocal_ScreenLocation))) (* (.x _returnvalue_2) 0.3)) (< (.X (Math|Vector2D|BreakVector2D (LocalVariables|GetLocal_ScreenLocation))) (* (.x _returnvalue_2) 0.7)) (> (.Y (Math|Vector2D|BreakVector2D (LocalVariables|GetLocal_ScreenLocation))) (* (.y _returnvalue_2) 0.2)) (< (.Y (Math|Vector2D|BreakVector2D (LocalVariables|GetLocal_ScreenLocation))) (* (.y _returnvalue_2) 0.8)))
        (if (LocalVariables|GetLocal_DoAction?)
          (Default|CalculeDistance (LocalVariables|GetLocal_PingRef) false)
          (Default|OnFade (LocalVariables|GetLocal_PingRef) true)
          (return true true)
          (else
            (return true true)))
        (else
          _)))
    (if (LocalVariables|GetLocal_DoAction?)
      (Default|CalculeDistance (LocalVariables|GetLocal_PingRef) false)
      (Default|OnFade (LocalVariables|GetLocal_PingRef) false))
    (return true false)
    (else
      (return false false))))